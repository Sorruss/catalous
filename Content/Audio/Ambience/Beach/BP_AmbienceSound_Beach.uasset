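; Beach ambience trigger actor that starts a looping-agnostic ambient sound when a qualifying actor enters its collision volume.
; The construction script assigns the configurable sound cue and attenuation settings to the audio component.
; On begin overlap, actors passing the BPI_MC_UI cast start playback at a random time within the cue's duration, varying each start.
; No end-overlap logic stops the sound.
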(event OnComponentBeginOverlap(CubeCollison)
  (params (OverlappedComponent :type Primitive%20Component%20Object%20Reference) (OtherActor :type Actor%20Object%20Reference) (OtherComp :type Primitive%20Component%20Object%20Reference) (OtherBodyIndex :type Integer) (bFromSweep :type Boolean) (SweepResult :type Hit%20Result%20Structure%20%28by%20ref%29))
  (Utilities|Casting|CastToBPI_MC_UI OtherActor)
  (Audio|Components|Audio|Play (Variables|Default|GetAmbienceBeach) (Math|Random|RandomFloatinRange 0.0 (Variables|/Script/Engine.SoundBase|GetDuration (Variables|Default|GetSoundCue)))))

(fn ConstructionScript
  (Audio|Components|Audio|SetSound (Variables|Default|GetAmbienceBeach) (Variables|Default|GetSoundCue))
  (Variables|/Script/Engine.AudioComponent|SetAttenuationSettings (Variables|Default|GetAmbienceBeach) (Variables|Default|GetAmbienceSoundAttenuation))
  (Variables|Default|SetCubeCollison (Variables|Default|GetCubeCollison))
  (Variables|Default|SetCubeSize (Variables|Default|GetCubeSize)))