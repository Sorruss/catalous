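; BP_Bonfire is an interactable bonfire with a named warp and spawn point that also burns whatever steps into it.
; Overlapping UsageCollision passes the bonfire's ID, name and transforms to actors implementing BPI_Interact and toggles their interact tip.
; Overlapping FireDamageCollision starts a looping timer that damages BPI_Damagable actors with interrupting hits, cleared on any end overlap.
; GetData exposes the bonfire's identity, screenshot and transforms.
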(event OnComponentBeginOverlap(UsageCollision)
  (params (OverlappedComponent :type Primitive%20Component%20Object%20Reference) (OtherActor :type Actor%20Object%20Reference) (OtherComp :type Primitive%20Component%20Object%20Reference) (OtherBodyIndex :type Integer) (bFromSweep :type Boolean) (SweepResult :type Hit%20Result%20Structure%20%28by%20ref%29))
  (if (Utilities|DoesObjectImplementInterface OtherActor "/Game/Catalous/Controls/Interfaces/BPI_Interact.BPI_Interact_C")
    (Class|BPIInteract|SetInteractionBonfireData(Message) OtherActor (Utilities|Struct|MakeS_InteractionBonfire (Transformation|GetWorldTransform (Variables|Default|GetSpawnLocation)) (Transformation|GetActorTransform) (Variables|Default|GetName) (Utilities|GetObjectName self) false))
    (Class|BPIInteract|ShowInteractTip(Message) OtherActor "NewEnumerator2" true)))

(event OnComponentEndOverlap(UsageCollision)
  (params (OverlappedComponent :type Primitive%20Component%20Object%20Reference) (OtherActor :type Actor%20Object%20Reference) (OtherComp :type Primitive%20Component%20Object%20Reference) (OtherBodyIndex :type Integer))
  (if (Utilities|DoesObjectImplementInterface OtherActor "/Game/Catalous/Controls/Interfaces/BPI_Interact.BPI_Interact_C")
    (Class|BPIInteract|ShowInteractTip(Message) OtherActor "NewEnumerator2" false)))

(event OnComponentBeginOverlap(FireDamageCollision)
  (params (OverlappedComponent :type Primitive%20Component%20Object%20Reference) (OtherActor :type Actor%20Object%20Reference) (OtherComp :type Primitive%20Component%20Object%20Reference) (OtherBodyIndex :type Integer) (bFromSweep :type Boolean) (SweepResult :type Hit%20Result%20Structure%20%28by%20ref%29))
  ;[0.15 0.15 0.15 0.5] Bonfire Stepon Damage Logic
  (if (Utilities|DoesObjectImplementInterface OtherActor "/Game/Catalous/Controls/Interfaces/BPI_Damagable.BPI_Damagable_C")
    (bind _returnvalue (Utilities|Time|SetTimerbyEvent (delegate Custom|FireDamageStart) 0.1 true))))

(event OnComponentEndOverlap(FireDamageCollision)
  (params (OverlappedComponent :type Primitive%20Component%20Object%20Reference) (OtherActor :type Actor%20Object%20Reference) (OtherComp :type Primitive%20Component%20Object%20Reference) (OtherBodyIndex :type Integer))
  ;[0.15 0.15 0.15 0.5] Bonfire Stepon Damage Logic
  (CallFunction|FireDamageEnd))

(event Custom|FireDamageEnd
  ;[0.15 0.15 0.15 0.5] Bonfire Stepon Damage Logic
  (if (Utilities|Time|IsValidTimerHandle (stale OnComponentBeginOverlap(FireDamageCollision) _returnvalue))
    (Utilities|Time|ClearandInvalidateTimerbyHandle (stale OnComponentBeginOverlap(FireDamageCollision) _returnvalue))))

(event Custom|FireDamageStart
  (bind _damageper (Variables|Default|GetDamagePer))
  ;[0.15 0.15 0.15 0.5] Bonfire Stepon Damage Logic
  (Class|BPIDamagable|GetDamaged(Message) (stale OnComponentBeginOverlap(FireDamageCollision) OtherActor) (Utilities|Struct|MakeS_DamageInfo self _damageper _damageper false false true false "NewEnumerator1")))

(fn ConstructionScript)

(fn GetData
  (return (Utilities|Struct|MakeS_Bonfire (Utilities|GetObjectName self) (Variables|Default|GetName) (Variables|Default|GetTexture) (Transformation|GetWorldTransform (Variables|Default|GetSpawnLocation)) (Transformation|GetActorTransform))))