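; BP_Pickable is a pickable item actor that shows an interact tip while another actor overlaps its collision box.
; On BeginPlay it selects the Niagara effect from PickableTier, with only one tier mapped to a pickup effect.
; It exposes its Category, while SetQuantity and the ammo, consumable, melee and ranged weapon data getters are empty stubs.
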(event OnComponentBeginOverlap(CollisionBox)
  (params (OverlappedComponent :type Primitive%20Component%20Object%20Reference) (OtherActor :type Actor%20Object%20Reference) (OtherComp :type Primitive%20Component%20Object%20Reference) (OtherBodyIndex :type Integer) (bFromSweep :type Boolean) (SweepResult :type Hit%20Result%20Structure%20%28by%20ref%29))
  (Class|BPIInteract|ShowInteractTip(Message) OtherActor true))

(event OnComponentEndOverlap(CollisionBox)
  (params (OverlappedComponent :type Primitive%20Component%20Object%20Reference) (OtherActor :type Actor%20Object%20Reference) (OtherComp :type Primitive%20Component%20Object%20Reference) (OtherBodyIndex :type Integer))
  (Class|BPIInteract|ShowInteractTip(Message) OtherActor false))

(event EventBeginPlay
  (Class|NiagaraComponent|SetAsset (Variables|Default|GetNiagara) (Utilities|Select :Index (Variables|Default|GetPickableTier) :NewEnumerator0 0 :NewEnumerator1 "/Game/Catalous/VFX/NS_PickUp_1.NS_PickUp_1" :NewEnumerator2 0 :NewEnumerator3 0) true))

(fn ConstructionScript)

(fn SetQuantity)

(fn GetAmmoData
  (return ""))

(fn GetCategory
  (return (Variables|Default|GetCategory)))

(fn GetConsumableData
  (return ""))

(fn GetWeaponMeleeData
  (return ""))

(fn GetWeaponRangedData
  (return ""))