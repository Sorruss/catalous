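; Ammo pickup actor that carries an ammo data struct describing what it holds.
; On BeginPlay, unless its Identifier is one excluded enum value, it looks up the DT_Ammo row named after that enum and caches it as AmmoData.
; Its SetQuantity override then calls the parent and writes Quantity into the cached struct, which GetAmmoData exposes.
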(event EventBeginPlay
  (|CallParentFunction)
  (if (Utilities|Enum|NotEqual(Enum) (Variables|Default|GetIdentifier) "NewEnumerator1")
    (bind _returnvalue (Utilities|GetDataTableRow "/Game/Catalous/Controls/DataTables/DT_Ammo.DT_Ammo" (Utilities|String|StringToName (Utilities|String|EnumtoString (Variables|Default|GetIdentifier))))
      (:then
        (Variables|Default|SetAmmoData _returnvalue)
        (CallFunction|SetQuantity)))))

(fn ConstructionScript
  (|CallParentFunction))

(fn GetAmmoData
  (return (Variables|Default|GetAmmoData)))

(fn SetQuantity
  (|CallParentFunction)
  (Utilities|Struct|SetmembersinS_Ammo (Variables|Default|GetAmmoData) (Variables|Default|GetQuantity)))