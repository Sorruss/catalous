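; BP_Pickable_Consumable is a pickable actor child class that represents a consumable item.
; On BeginPlay, unless Identifier is the first enum entry, it converts the enum to a row name, loads that DT_Consumables row into ConsumableData and calls SetQuantity.
; The SetQuantity override runs the parent logic, then writes Quantity into the struct.
; GetConsumableData also applies Quantity before returning the struct.
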(event EventBeginPlay
  (|CallParentFunction)
  (if (Utilities|Enum|NotEqual(Enum) (Variables|Default|GetIdentifier) "NewEnumerator0")
    (bind _returnvalue (Utilities|GetDataTableRow "/Game/Catalous/Controls/DataTables/DT_Consumables.DT_Consumables" (Utilities|String|StringToName (Utilities|String|EnumtoString (Variables|Default|GetIdentifier))))
      (:then
        (Variables|Default|SetConsumableData _returnvalue)
        (CallFunction|SetQuantity)))))

(fn ConstructionScript
  (|CallParentFunction))

(fn GetConsumableData
  (bind _structout (Utilities|Struct|SetmembersinS_Consumables (Variables|Default|GetConsumableData) (Variables|Default|GetQuantity)))
  (return _structout))

(fn SetQuantity
  (|CallParentFunction)
  (Utilities|Struct|SetmembersinS_Consumables (Variables|Default|GetConsumableData) (Variables|Default|GetQuantity)))