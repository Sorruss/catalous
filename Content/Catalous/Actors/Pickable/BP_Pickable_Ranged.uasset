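; Pickable actor for a ranged weapon that carries that weapon's data.
; On BeginPlay, after the parent logic, it converts the WeaponID enum to a row name, skipping the first enumerator.
; It caches the matching DT_WeaponRanged row in WeaponData, which GetWeaponRangedData returns to callers.
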(event EventBeginPlay
  (|CallParentFunction)
  (if (Utilities|Enum|NotEqual(Enum) (Variables|Default|GetWeaponID) "NewEnumerator0")
    (bind _returnvalue (Utilities|GetDataTableRow "/Game/Catalous/Controls/DataTables/DT_WeaponRanged.DT_WeaponRanged" (Utilities|String|StringToName (Utilities|String|EnumtoString (Variables|Default|GetWeaponID))))
      (:then
        (Variables|Default|SetWeaponData _returnvalue)))))

(fn ConstructionScript
  (|CallParentFunction))

(fn GetWeaponRangedData
  (return (Variables|Default|GetWeaponData)))