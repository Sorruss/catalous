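; BP_Pickable_Ring is a pickable ring actor that carries the data for one ring type.
; On BeginPlay it runs the parent logic, then, unless RingID is one excluded enum value, looks up the matching DT_Ring row using the enum's string as the row name.
; The found row is cached in RingData, which GetRingData returns.
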(event EventBeginPlay
  (|CallParentFunction)
  (if (Utilities|Enum|NotEqual(Enum) (Variables|Default|GetRingID) "NewEnumerator4")
    (bind _returnvalue (Utilities|GetDataTableRow "/Game/Catalous/Controls/DataTables/DT_Ring.DT_Ring" (Utilities|String|StringToName (Utilities|String|EnumtoString (Variables|Default|GetRingID))))
      (:then
        (Variables|Default|SetRingData _returnvalue)))))

(fn ConstructionScript
  (|CallParentFunction))

(fn GetRingData
  (return (Variables|Default|GetRingData)))