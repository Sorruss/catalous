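; BP_Pickable_StarterSword is a pickable actor for the starter melee sword.
; On BeginPlay, after the parent logic, it skips one specific WeaponID value and otherwise uses the ID's enum name as a row name in DT_WeaponMelee.
; A found row is cached in WeaponData, which GetWeaponMeleeData returns to callers.
; The construction script only runs the parent's.
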(event EventBeginPlay
  (|CallParentFunction)
  (if (Utilities|Enum|NotEqual(Enum) (Variables|Default|GetWeaponID) "NewEnumerator1")
    (bind _returnvalue (Utilities|GetDataTableRow "/Game/Catalous/Controls/DataTables/DT_WeaponMelee.DT_WeaponMelee" (Utilities|String|StringToName (Utilities|String|EnumtoString (Variables|Default|GetWeaponID))))
      (:then
        (Variables|Default|SetWeaponData _returnvalue)))))

(fn ConstructionScript
  (|CallParentFunction))

(fn GetWeaponMeleeData
  (return (Variables|Default|GetWeaponData)))