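; Generic enemy and boss character that destroys itself on spawn if the game instance has its death saved.
; Damage component events drive floating or boss health bars, poise-break reactions, and death with ragdoll and souls reward.
; Montage notifies chain and delay ADR attack combos, run sequentially or picked recursively by distance-weighted probability.
; It also handles backstab detection, evade chance, healing on player death, and teleporting as invisible, high-speed flying AI movement.
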(event OnComponentBeginOverlap(BackStab)
  (params (OverlappedComponent :type Primitive%20Component%20Object%20Reference) (OtherActor :type Actor%20Object%20Reference) (OtherComp :type Primitive%20Component%20Object%20Reference) (OtherBodyIndex :type Integer) (bFromSweep :type Boolean) (SweepResult :type Hit%20Result%20Structure%20%28by%20ref%29))
  ;[0.15 0.15 0.15 0.5] Backstab Logic
  (if (Actor|ActorHasTag OtherActor "MC")
    (Default|ChangeColor (Variables|Default|GetWBP%20LockOnCircle) "NewEnumerator2")
    (Variables|Default|SetIsBackstabbable? true)))

(event OnComponentEndOverlap(BackStab)
  (params (OverlappedComponent :type Primitive%20Component%20Object%20Reference) (OtherActor :type Actor%20Object%20Reference) (OtherComp :type Primitive%20Component%20Object%20Reference) (OtherBodyIndex :type Integer))
  ;[0.15 0.15 0.15 0.5] Backstab Logic
  (if (Actor|ActorHasTag OtherActor "MC")
    (Default|ChangeColor (Variables|Default|GetWBP%20LockOnCircle) "NewEnumerator1")
    (Variables|Default|SetIsBackstabbable? false)))

(event Custom|OnPoiseBreak
  (params (Direction :type E_HitDirection%20Enum :default "NewEnumerator0"))
  ;[0.15 0.15 0.15 0.5] Damage System Logic
  (Variables|/Script/Engine.CharacterMovementComponent|SetMaxWalkSpeed (Variables|Character|GetCharacterMovement) 0.0)
  (Animation|StopAnimMontage 0)
  (Animation|Montage|PlayMontage (Variables|Character|GetMesh) (Utilities|Select :Index Direction :NewEnumerator0 "/Game/Catalous/Characters/Enemies/SkeletonMelee/Animations/HitReaction/Anim_SwordV2_Hit_Big_F_IP_Montage.Anim_SwordV2_Hit_Big_F_IP_Montage" :NewEnumerator1 "/Game/Catalous/Characters/Enemies/SkeletonMelee/Animations/HitReaction/Anim_SwordV2_Hit_Big_F_IP_Montage.Anim_SwordV2_Hit_Big_F_IP_Montage" :NewEnumerator2 "/Game/Catalous/Characters/Enemies/SkeletonMelee/Animations/HitReaction/Anim_SwordV2_Hit_Big_L_IP_Montage.Anim_SwordV2_Hit_Big_L_IP_Montage" :NewEnumerator3 "/Game/Catalous/Characters/Enemies/SkeletonMelee/Animations/HitReaction/Anim_SwordV2_Hit_Big_R_IP_Montage.Anim_SwordV2_Hit_Big_R_IP_Montage" :NewEnumerator6 "/Game/Catalous/Characters/Enemies/SkeletonMelee/Animations/HitReaction/Anim_SwordV2_Hit_Big_B_IP_Montage.Anim_SwordV2_Hit_Big_B_IP_Montage") 0.6
    (:OnCompleted
      _)
    (:OnInterrupted
      _))
  (CallFunction|SetMovementSpeed "NewEnumerator1"))

(event Custom|OnDamage
  (params (NewHP :type Float%20%28double-precision%29))
  ;[0.15 0.15 0.15 0.5] Damage System Logic
  (CallFunction|UpdateHPBar)
  (Audio|PlaySoundatLocation "/Game/Catalous/SFX/Combat/Damaged2.Damaged2" (Transformation|GetActorLocation) "0, 0, 0" 0.35 1.0 0.0 0 0 0 0))

(event Custom|ShowHealthBarRetrig
  (params (Damager :type Object%20Object%20Reference))
  ;[0.15 0.15 0.15 0.5] HealthBar Visibility Logic
  (Variables|/Script/UMG.Widget|SetRenderOpacity (Variables|Default|GetWBP%20Health%20Bar) 1.0)
  (Utilities|FlowControl|RetriggerableDelay 5.0)
  (bind _islockedon (Class|BPIMCUI|GetIsLockedon(Message) Damager))
  (if (not _islockedon)
    (Variables|/Script/UMG.Widget|SetRenderOpacity (Variables|Default|GetWBP%20Health%20Bar) 0.0)))

(event Custom|ShowHealthBarBoss
  (params (Show? :type Boolean) (Anim? :type Boolean))
  ;[0.15 0.15 0.15 0.5] HealthBar Visibility Logic
  (Widget|SetVisibility (Variables|Default|GetWBP%20BossHealthBar) (select Show? "Visible" "Hidden")))

(event Custom|TeleportStart
  (params (Destination :type Vector))
  (bind _charactermovement (Variables|Character|GetCharacterMovement))
  ;[0.15 0.15 0.15 0.5] Teleportation Logic
  (if (not (Variables|Default|GetIsTeleporting?))
    (Pawn|Components|CharacterMovement|SetMovementMode _charactermovement "MOVE_Flying" 0)
    (Variables|/Script/Engine.CharacterMovementComponent|SetMaxFlySpeed _charactermovement 5e+03)
    (Variables|/Script/Engine.CharacterMovementComponent|SetMaxAcceleration _charactermovement 99999.0)
    (Rendering|SetVisibility (Variables|Character|GetMesh) false true)
    (Collision|SetCollisionResponsetoChannel (Variables|Default|GetCapsuleComponent) "ECC_Pawn" "ECR_Ignore")
    (bind _returnvalue (Effects|SpawnEmitterAttached 0 (Variables|Character|GetMesh) "spine_02"))
    (Variables|Default|SetTeleportEmitter1 _returnvalue)
    (bind _returnvalue_2 (Effects|SpawnEmitterAttached 0 (Variables|Character|GetMesh) "spine_02"))
    (Variables|Default|SetTeleportEmitter2 _returnvalue_2)
    (Animation|StopAnimMontage 0)
    (AI|AIMoveTo self Destination 0 (Variables|Default|GetAttack%20Range) false
      (:OnSuccess
        _)
      (:OnFail
        _))
    (CallFunction|TeleportEnd)
    (else
      (Utilities|FlowControl|DelayUntilNextTick)
      (Default|CallOnTeleportEnd))))

(event Custom|TeleportEnd
  (bind _charactermovement (Variables|Character|GetCharacterMovement))
  ;[0.15 0.15 0.15 0.5] Teleportation Logic
  (Components|Movement|StopMovementImmediately _charactermovement)
  (Pawn|Components|CharacterMovement|SetMovementMode _charactermovement "MOVE_Walking" 0)
  (Variables|/Script/Engine.CharacterMovementComponent|SetMaxFlySpeed _charactermovement 5e+03)
  (Variables|/Script/Engine.CharacterMovementComponent|SetMaxAcceleration _charactermovement 1.5e+03)
  (Rendering|SetVisibility (Variables|Character|GetMesh) true true)
  (Collision|SetCollisionResponsetoChannel (Variables|Default|GetCapsuleComponent) "ECC_Pawn" "ECR_Block")
  (Default|CallOnTeleportEnd)
  (Utilities|FlowControl|Delay 0.5)
  (bind _teleportemitter1 (Variables|Default|GetTeleportEmitter1)
    (:then
      (Components|DestroyComponent _teleportemitter1))
    (:else
      _))
  (bind _teleportemitter2 (Variables|Default|GetTeleportEmitter2)
    (:then
      (Components|DestroyComponent _teleportemitter2))
    (:else)))

(event Custom|NextADR
  (bind _mesh (Variables|Character|GetMesh))
  (bind _returnvalue (Components|SkeletalMesh|GetAnimInstance _mesh))
  ;[0.15 0.15 0.15 0.5] ADR Logic
  (Variables|Default|SetIsMontage? true)
  (Variables|Default|SetIsAttacking? true)
  (Variables|Default|SetADRLastAttack? (== (- (Utilities|Array|Length (.AttackDelay (Utilities|Struct|BreakS_AttackDelayRest (Utilities|Array|Get(acopy) (Variables|Default|GetADRs) (Variables|Default|GetCurrentADRCount))))) 1) (Variables|Default|GetCurrentAttackCount)))
  (bind _notifyname (Animation|Montage|PlayMontage (Variables|Character|GetMesh) (.AttackMontage (Utilities|Struct|BreakS_AttackDelay (Utilities|Array|Get(acopy) (.AttackDelay (Utilities|Struct|BreakS_AttackDelayRest (Utilities|Array|Get(acopy) (Variables|Default|GetADRs) (Variables|Default|GetCurrentADRCount)))) (Variables|Default|GetCurrentAttackCount)))))
    (:OnNotifyBegin
      (switch name _notifyname
        (:NextAttack
          (if (not (Variables|Default|GetADRLastAttack?))
            (Math|Integer|IncrementInt (Variables|Default|GetCurrentAttackCount)
              (:%20%20
                (CallFunction|NextADR)))
            (else
              (Variables|Default|SetCurrentAttackCount 0)
              (bind _newvalue (CallFunction|IncreaseIntLoop (Variables|Default|GetCurrentADRCount) 1 (- (Utilities|Array|Length (Variables|Default|GetADRs)) 1)))
              (Variables|Default|SetCurrentADRCount _newvalue)
              (Default|CallOnMontageFinish (.Rest (Utilities|Struct|BreakS_AttackDelayRest (Utilities|Array|Get(acopy) (Variables|Default|GetADRs) (Variables|Default|GetCurrentADRCount)))))
              (Variables|Default|SetIsMontage? false)
              (Variables|Default|SetIsAttacking? false))))
        (:Delay
          (Animation|Montage|MontageSetPlayRate _returnvalue (.AttackMontage (Utilities|Struct|BreakS_AttackDelay (Utilities|Array|Get(acopy) (.AttackDelay (Utilities|Struct|BreakS_AttackDelayRest (Utilities|Array|Get(acopy) (Variables|Default|GetADRs) (Variables|Default|GetCurrentADRCount)))) (Variables|Default|GetCurrentAttackCount)))) 0.3)
          (Utilities|FlowControl|Delay (.Delay (Utilities|Struct|BreakS_AttackDelay (Utilities|Array|Get(acopy) (.AttackDelay (Utilities|Struct|BreakS_AttackDelayRest (Utilities|Array|Get(acopy) (Variables|Default|GetADRs) (Variables|Default|GetCurrentADRCount)))) (Variables|Default|GetCurrentAttackCount)))))
          (Animation|Montage|MontageSetPlayRate _returnvalue (.AttackMontage (Utilities|Struct|BreakS_AttackDelay (Utilities|Array|Get(acopy) (.AttackDelay (Utilities|Struct|BreakS_AttackDelayRest (Utilities|Array|Get(acopy) (Variables|Default|GetADRs) (Variables|Default|GetCurrentADRCount)))) (Variables|Default|GetCurrentAttackCount)))) 1.0))))))

(event Custom|UpdateHPBar
  ;[0.15 0.15 0.15 0.5] Damage System Logic
  (Default|ValueChanged (select (Variables|Default|GetBoss?) (Variables|/Game/Catalous/UI/Components/ProgressBar/WBP_HealthBar.WBP_HealthBar_C|GetWCBP_Generic_ProgressBar (Variables|/Game/Catalous/UI/Components/ProgressBar/WBP_Boss_HealthBar.WBP_Boss_HealthBar_C|GetWBP_HealthBar (Variables|Default|GetWBP%20BossHealthBar))) (Variables|/Game/Catalous/UI/Components/ProgressBar/WBP_HealthBar.WBP_HealthBar_C|GetWCBP_Generic_ProgressBar (Variables|Default|GetWBP%20Health%20Bar)))))

(event Custom|Set%20LockOn%20Sprite%20Position
  ;[0.15 0.15 0.15 0.5] Placing Widgets At Nice Places
  (Transformation|AddLocalOffset (Variables|Default|GetWBP_LockOnCircle) (Math|Vector|MakeVector 0.0 0.0 (* (.z (.BoxExtent (Collision|GetComponentBounds (Variables|Character|GetMesh)))) (Variables|Default|GetDelta%20LockOn%20Widget%20Height))) false false))

(event Custom|OnBlock
  (params (NewHP :type Float%20%28double-precision%29) (StaminaReq :type Float%20%28double-precision%29))
  ;[0.15 0.15 0.15 0.5] Damage System Logic
  (CallFunction|UpdateHPBar)
  (Audio|PlaySoundatLocation "/Game/Catalous/SFX/Combat/Damaged2.Damaged2" (Transformation|GetActorLocation) "0, 0, 0" 0.35 1.0 0.0 0 0 0 0))

(event Custom|OnEvade
  ;[0.15 0.15 0.15 0.5] Damage System Logic
)

(event Custom|OnDeath
  ;[0.15 0.15 0.15 0.5] Damage System Logic
  (CallFunction|OnDeathResponse)
  (CallFunction|UpdateHPBar)
  (Class|BPISaveGame|SaveEnemybyID(Message) (Game|GetGameInstance) (Utilities|GetObjectName self) true)
  (Audio|PlaySoundatLocation (Variables|Default|GetDeathSound) (Transformation|GetActorLocation) "0, 0, 0" 0.5 1.0 0.0 0 0 0 0)
  (Utilities|FlowControl|Delay (Variables|Default|GetLifespanAfterDeath))
  (Actor|DestroyActor)
  (CallFunction|AfterLifespanEnd))

(event Custom|Set%20HealthBar%20Position
  ;[0.15 0.15 0.15 0.5] Placing Widgets At Nice Places
  (Transformation|AddLocalOffset (Variables|Default|GetWBP_HealthBar) (Math|Vector|MakeVector 0.0 0.0 (* (.z (.BoxExtent (Collision|GetComponentBounds (Variables|Character|GetMesh)))) (Variables|Default|GetDelta%20HealthBar%20Widget%20Height))) false false))

(event Custom|Init%20Widgets%20Values
  ;[0.15 0.15 0.15 0.5] Widget Initializing
  (bind _aswbp_health_bar (Utilities|Casting|CastToWBP_HealthBar (UserInterface|GetWidget (Variables|Default|GetWBP_HealthBar))))
  (bind _output_get (Variables|Default|SetWBP%20Health%20Bar _aswbp_health_bar))
  (Variables|/Game/Catalous/UI/Components/ProgressBar/WBP_HealthBar.WBP_HealthBar_C|SetOwner _output_get self)
  (Default|Initialize _output_get)
  (Default|UpdateNoAnim _output_get)
  (CallFunction|ShowHealthBarWidget false false))

(event Custom|RandomADR
  (params (Index :type Integer))
  (bind _returnvalue (!= Index -1))
  (bind _mesh (Variables|Character|GetMesh))
  (bind _returnvalue_2 (Components|SkeletalMesh|GetAnimInstance _mesh))
  ;[0.15 0.15 0.15 0.5] Random ADRPD Logic
  (if _returnvalue
    _
    (else
      (bind (_index _adr) (CallFunction|GetRandomADRPD))))
  (Variables|Default|SetIsMontage? true)
  (Variables|Default|SetIsAttacking? true)
  (Variables|Default|SetADRLastAttack? (== (- (Utilities|Array|Length (.AttackDelay (Utilities|Struct|BreakS_AttackDelayRest (select _returnvalue (Utilities|Array|Get(acopy) (Variables|Default|GetADRs) Index) _adr)))) 1) (Variables|Default|GetCurrentAttackCount)))
  (bind _notifyname (Animation|Montage|PlayMontage (Variables|Character|GetMesh) (.AttackMontage (Utilities|Struct|BreakS_AttackDelay (Utilities|Array|Get(acopy) (.AttackDelay (Utilities|Struct|BreakS_AttackDelayRest (select _returnvalue (Utilities|Array|Get(acopy) (Variables|Default|GetADRs) Index) _adr))) (Variables|Default|GetCurrentAttackCount)))))
    (:OnNotifyBegin
      (switch name _notifyname
        (:NextAttack
          (if (not (Variables|Default|GetADRLastAttack?))
            (Math|Integer|IncrementInt (Variables|Default|GetCurrentAttackCount)
              (:%20%20
                (CallFunction|RandomADR (Math|Integer|SelectInt Index _index _returnvalue))))
            (else
              (Variables|Default|SetCurrentAttackCount 0)
              (Default|CallOnMontageFinish (.Rest (Utilities|Struct|BreakS_AttackDelayRest (select _returnvalue (Utilities|Array|Get(acopy) (Variables|Default|GetADRs) Index) _adr))))
              (Variables|Default|SetIsMontage? false)
              (Variables|Default|SetIsAttacking? false))))
        (:Delay
          (Animation|Montage|MontageSetPlayRate _returnvalue_2 (.AttackMontage (Utilities|Struct|BreakS_AttackDelay (Utilities|Array|Get(acopy) (.AttackDelay (Utilities|Struct|BreakS_AttackDelayRest (select _returnvalue (Utilities|Array|Get(acopy) (Variables|Default|GetADRs) Index) _adr))) (Variables|Default|GetCurrentAttackCount)))) 0.3)
          (Utilities|FlowControl|Delay (.Delay (Utilities|Struct|BreakS_AttackDelay (Utilities|Array|Get(acopy) (.AttackDelay (Utilities|Struct|BreakS_AttackDelayRest (select _returnvalue (Utilities|Array|Get(acopy) (Variables|Default|GetADRs) Index) _adr))) (Variables|Default|GetCurrentAttackCount)))))
          (Animation|Montage|MontageSetPlayRate _returnvalue_2 (.AttackMontage (Utilities|Struct|BreakS_AttackDelay (Utilities|Array|Get(acopy) (.AttackDelay (Utilities|Struct|BreakS_AttackDelayRest (select _returnvalue (Utilities|Array|Get(acopy) (Variables|Default|GetADRs) Index) _adr))) (Variables|Default|GetCurrentAttackCount)))) 1.0))))))

(event Custom|Init%20BossHealthBar
  ;[0.15 0.15 0.15 0.5] HealthBar Visibility Logic
  (bind _returnvalue (UserInterface|CreateWidget "/Game/Catalous/UI/Components/ProgressBar/WBP_Boss_HealthBar.WBP_Boss_HealthBar_C" (Game|GetPlayerController 0) (Utilities|Text|ToText(String) (Utilities|String|EnumtoString (Utilities|Struct|BreakS_Character (Variables|Default|GetCharacterStruct))))))
  (bind _output_get (Variables|Default|SetWBP%20BossHealthBar _returnvalue))
  (UserInterface|Viewport|AddtoViewport _output_get 0)
  (Variables|/Game/Catalous/UI/Components/ProgressBar/WBP_HealthBar.WBP_HealthBar_C|SetOwner (Variables|/Game/Catalous/UI/Components/ProgressBar/WBP_Boss_HealthBar.WBP_Boss_HealthBar_C|GetWBP_HealthBar _output_get) self)
  (Default|Initialize (Variables|/Game/Catalous/UI/Components/ProgressBar/WBP_Boss_HealthBar.WBP_Boss_HealthBar_C|GetWBP_HealthBar _output_get))
  (Default|UpdateNoAnim (Variables|/Game/Catalous/UI/Components/ProgressBar/WBP_Boss_HealthBar.WBP_Boss_HealthBar_C|GetWBP_HealthBar _output_get)))

(event Custom|ShowHealthBar
  (params (Show? :type Boolean) (Anim? :type Boolean))
  ;[0.15 0.15 0.15 0.5] HealthBar Visibility Logic
  (if Show?
    (Utilities|FlowControl|Sequence
      (:then_0
        (bind _alpha (Timeline|Timeline Stop)
          (:Update
            (Variables|/Script/UMG.Widget|SetRenderOpacity (Variables|Default|GetWBP%20Health%20Bar) _alpha))))
      (:then_1
        (Variables|/Script/UMG.Widget|SetRenderOpacity (Variables|Default|GetWBP%20Health%20Bar) 1.0)))
    (elif Anim?
      (Timeline|Timeline PlayFromStart)
      (else
        (Variables|/Script/UMG.Widget|SetRenderOpacity (Variables|Default|GetWBP%20Health%20Bar) 0.0)))))

(event EventBeginPlay
  (bind _shouldbedestroyed_ (Class|BPISaveGame|GetEnemybyID(Message) (Game|GetGameInstance) (Utilities|GetObjectName self)))
  (if _shouldbedestroyed_
    (Variables|Default|SetDestroyedOnStart? true)
    (Actor|DestroyActor)
    (else
      (|CallParentFunction)
      (CallFunction|SetLockonSpritePosition)
      (bind _aswbp_lock_on_circle (Utilities|Casting|CastToWBP_LockOnCircle (UserInterface|GetWidget (Variables|Default|GetWBP_LockOnCircle))))
      (Variables|Default|SetWBP%20LockOnCircle _aswbp_lock_on_circle)
      (bind _asaic_enemy_base (Utilities|Casting|CastToAIC_Enemy_Base (AI|GetAIController self)))
      (Variables|Default|SetAIController0 _asaic_enemy_base)
      (bind _asbp_knight (Utilities|Casting|CastToBP_Knight (Game|GetPlayerCharacter 0)))
      (EventDispatchers|BindEventtoOnDeath (Variables|/Game/Catalous/Characters/MC/BP_Knight.BP_Knight_C|GetAC_DamageSystem _asbp_knight) (EventDispatchers|CreateEvent :!event OnPlayerDeath))
      (if (not (Variables|Default|GetBoss?))
        (CallFunction|SetHealthBarPosition)
        (CallFunction|InitWidgetsValues)
        (else
          (CallFunction|InitBossHealthBar)
          (CallFunction|ShowHealthBarBoss false false)
          (Components|DestroyComponent (Variables|Default|GetWBP_HealthBar)))))))

(event EventTeleport
  (params (Destination :type Vector :default "0, 0, 0"))
  ;[0.15 0.15 0.15 0.5] Teleportation Logic
  (CallFunction|TeleportStart Destination))

(event EventShowHealthBarWidgetRetriggerable
  (params (Damager :type Actor%20Object%20Reference))
  ;[0.15 0.15 0.15 0.5] HealthBar Visibility Logic
  (if (not (Variables|Default|GetBoss?))
    (CallFunction|ShowHealthBarRetrig Damager)))

(event EventStartAOETrace
  (params (Radius :type Float%20%28double-precision%29))
  (Default|AOETrace (Variables|Default|GetAC_AttackSystem_AI) Radius))

(event EventPlayBackstab
  (params (SubType :type E_WeaponSubtype%20Enum :default "NewEnumerator0"))
  (Variables|Default|SetIsMontage? true)
  (Animation|Montage|PlayMontage (Variables|Character|GetMesh) (Utilities|Select :Index SubType :NewEnumerator0 0 :NewEnumerator1 0 :NewEnumerator2 "/Game/Catalous/Characters/Enemies/SkeletonMelee/Animations/A_Stealthkillvictem_Montage.A_Stealthkillvictem_Montage" :NewEnumerator3 "/Game/Catalous/Characters/Enemies/SkeletonMelee/Animations/GreatSword_Attack_Ambushed_Montage.GreatSword_Attack_Ambushed_Montage" :NewEnumerator4 0 :NewEnumerator5 "/Game/Catalous/Characters/Enemies/SkeletonMelee/Animations/A_Stealthkillvictem_Montage.A_Stealthkillvictem_Montage" :NewEnumerator6 0)))

(event EventShowHealthBarWidget
  (params (Show? :type Boolean) (Anim? :type Boolean))
  ;[0.15 0.15 0.15 0.5] HealthBar Visibility Logic
  (if (not (Variables|Default|GetBoss?))
    (CallFunction|ShowHealthBar Show? Anim?)
    (else
      (CallFunction|ShowHealthBarBoss Show? Anim?))))

(fn ConstructionScript
  (bind _ac_damagesystem (Variables|Default|GetAC_DamageSystem))
  (|CallParentFunction)
  (EventDispatchers|BindEventtoOnDamage _ac_damagesystem (EventDispatchers|CreateEvent :!event Custom|OnDamage))
  (EventDispatchers|BindEventtoOnBlock _ac_damagesystem (EventDispatchers|CreateEvent :!event Custom|OnBlock))
  (EventDispatchers|BindEventtoOnEvade _ac_damagesystem (EventDispatchers|CreateEvent :!event Custom|OnEvade))
  (EventDispatchers|BindEventtoOnDeath _ac_damagesystem (EventDispatchers|CreateEvent :!event Custom|OnDeath))
  (EventDispatchers|BindEventtoOnPoiseBreak _ac_damagesystem (EventDispatchers|CreateEvent :!event Custom|OnPoiseBreak)))

(fn EnableRagdoll
  (Physics|SetSimulatePhysics (Variables|Character|GetMesh) true)
  (Pawn|UnPossess (AI|GetAIController self)))

(fn IncreaseIntLoop
  (params (IntVariable :type Integer) (IncreaseValue :type Integer) (Max :type Integer) (Min :type Integer))
  (if (> (+ IntVariable IncreaseValue) Max)
    (return Min)
    (else
      (return (+ IntVariable IncreaseValue)))))

(fn OnAbortRealodWeapon)

(fn GetWeaponActor
  (return 0))

(fn OnDeathResponse
  (bind _returnvalue (Game|Player|GetPlayerPawn 0))
  (bind _ac_attacksystem_ai (Variables|Default|GetAC_AttackSystem_AI))
  (Animation|StopAnimMontage 0)
  (CallFunction|EnableRagdoll)
  (Collision|SetCollisionEnabled (Variables|Default|GetCapsuleComponent) "NoCollision")
  (if (not (Variables|Default|GetBoss?))
    (CallFunction|ShowHealthBarWidget false false)
    (else
      (CallFunction|ShowHealthBarBoss false false)))
  (Class|BPIMCUI|GainSouls(Message) _returnvalue (.souls (Variables|Default|GetDropOnDeath)))
  (Class|BPIDamagable|SetTargetedbyAI(Message) _returnvalue false)
  (Components|DestroyComponent (Variables|Default|GetBackStab))
  (Components|DestroyComponent (Variables|Default|GetEvadeBox))
  (Default|EndMeleeDamageTrace _ac_attacksystem_ai)
  (Default|EndCloseCombatTrace _ac_attacksystem_ai))

(fn AfterLifespanEnd)

(fn Reset
  (bind _aicontroller0 (Variables|Default|GetAIController0))
  (Transformation|SetActorLocation (Variables|/Game/Catalous/Characters/Enemies/AI/AIC_Enemy_Base.AIC_Enemy_Base_C|GetStartLocation (Variables|Default|GetAIController0)) false false)
  (Utilities|IsValid (Variables|Default|GetPatrolRoute)
    (:Is%20Valid
      (Default|SetStateasPatrol _aicontroller0))
    (:Is%20Not%20Valid
      (Default|SetStateasIdle _aicontroller0))))

(fn GetRandomADRPD
  (bind _adrs (Variables|Default|GetADRs))
  (bind _output_get (LocalVariables|SetADRIndex (Math|Random|RandomIntegerinRange 0 (- (Utilities|Array|Length _adrs) 1))))
  (bind _output_get_2 (LocalVariables|SetADRPD (Utilities|Array|Get(acopy) _adrs _output_get)))
  (if (Math|Random|RandomBoolwithWeight (* (.Probability (Utilities|Struct|BreakS_AttackDelayRest _output_get_2)) (Math|Float|SelectFloat (/ (.Distance (Utilities|Struct|BreakS_AttackDelayRest _output_get_2)) (Transformation|GetDistanceTo (Variables|/Game/Catalous/Characters/Enemies/AI/AIC_Enemy_Base.AIC_Enemy_Base_C|GetTargetActor (Variables|Default|GetAIController0)))) (- 1.0 (- (/ (.Distance (Utilities|Struct|BreakS_AttackDelayRest _output_get_2)) (Transformation|GetDistanceTo (Variables|/Game/Catalous/Characters/Enemies/AI/AIC_Enemy_Base.AIC_Enemy_Base_C|GetTargetActor (Variables|Default|GetAIController0)))) 1.0)) (< (/ (.Distance (Utilities|Struct|BreakS_AttackDelayRest _output_get_2)) (Transformation|GetDistanceTo (Variables|/Game/Catalous/Characters/Enemies/AI/AIC_Enemy_Base.AIC_Enemy_Base_C|GetTargetActor (Variables|Default|GetAIController0)))) 1.0))))
    (return (LocalVariables|GetADRIndex) (LocalVariables|GetADRPD))
    (else
      (bind (_index _adr) (CallFunction|GetRandomADRPD))
      (return _index _adr))))

(fn OnPlayerDeath
  (Default|HealPercentage (Variables|Default|GetAC_DamageSystem) 1e+02)
  (Default|UpdateNoAnim (select (Variables|Default|GetBoss?) (Variables|/Game/Catalous/UI/Components/ProgressBar/WBP_Boss_HealthBar.WBP_Boss_HealthBar_C|GetWBP_HealthBar (Variables|Default|GetWBP%20BossHealthBar)) (Variables|Default|GetWBP%20Health%20Bar))))

(fn EndCloseCombatTrace)

(fn EndDamageTrace
  (Default|EndMeleeDamageTrace (Variables|Default|GetAC_AttackSystem_AI)))

(fn EndTrail)

(fn GetCharacterName
  (return (Variables|Default|GetCharacterName)))

(fn GetBlockingWeaponStats
  (return ""))

(fn GetDamaged
  (params (DamageInfo :type S%20Damage%20Info%20Structure))
  (bind _instigator (Utilities|Struct|BreakS_DamageInfo DamageInfo))
  (if (Utilities|ClassIsChildOf (Utilities|GetClass _instigator) "/Game/Catalous/Characters/MC/BP_Knight.BP_Knight_C")
    (if (not (Variables|Default|GetBoss?))
      (CallFunction|ShowHealthBarWidgetRetriggerable _instigator)
      (else
        (CallFunction|ShowHealthBarBoss true false))))
  (Default|GetDamaged (Variables|Default|GetAC_DamageSystem) DamageInfo)
  (return))

(fn GetDamagedActorState
  (return ""))

(fn GetHealthRatio
  (return (Default|GetHealthRatio (Variables|Default|GetAC_DamageSystem))))

(fn GetIsAttacking
  (return (Variables|Default|GetIsAttacking?)))

(fn GetIsBackstabbable?
  (return (Variables|Default|GetIsBackstabbable?)))

(fn GetMeleeWeaponActor
  (return 0))

(fn GetPatrolRoute
  (return (Variables|Default|GetPatrolRoute)))

(fn GetPrimaryasRanged
  (return 0))

(fn GetRanges
  (return (Variables|Default|GetAttack%20Range) (Variables|Default|GetStrafe%20Range) (Variables|Default|GetLooseRange)))

(fn HasEnoughStamina?
  (params (StaminaReq :type Float%20%28double-precision%29))
  (return false))

(fn Heal
  (params (Amount :type Float%20%28double-precision%29))
  (bind (_success _newamount) (Default|Heal (Variables|Default|GetAC_DamageSystem) Amount))
  (return _success _newamount))

(fn IsBoss?
  (return (Variables|Default|GetBoss?)))

(fn IsPrimaryEquiped?
  (return (Variables|Default|GetPrimaryEquiped?)))

(fn IsSecondaryEquipped?
  (return (Variables|Default|GetSecondaryEquipped?)))

(fn SetMovementSpeed
  (params (MovementSpeed :type E_MovementSpeed%20Enum :default "NewEnumerator0"))
  (bind _characterstruct (Variables|Default|GetCharacterStruct))
  (bind (_walkspeed _jogspeed _runspeed) (Utilities|Struct|BreakS_Character _characterstruct))
  (Variables|/Script/Engine.CharacterMovementComponent|SetMaxWalkSpeed (Variables|Character|GetCharacterMovement) (Utilities|Select :Index MovementSpeed :NewEnumerator0 0.0 :NewEnumerator1 _walkspeed :NewEnumerator2 _jogspeed :NewEnumerator3 _runspeed)))

(fn ShowLockonWidget
  (params (Show? :type Boolean))
  (Rendering|SetVisibility (Variables|Default|GetWBP_LockOnCircle) Show? false))

(fn StartCloseCombatTrace
  (params (BodyPart :type E_BodyParts%20Enum :default "NewEnumerator0")))

(fn StartDamageTrace
  (Default|StartMeleeDamageTrace (Variables|Default|GetAC_AttackSystem_AI)))

(fn StartTrail
  (params (Trail :type Niagara%20System%20Object%20Reference)))

(fn WillEvade?
  (bind _aicontroller0 (Variables|Default|GetAIController0)
    (:then
      (if (and (Utilities|Enum|Equal(Enum) (Default|GetCurrentState _aicontroller0) "NewEnumerator2") (not (Variables|Default|GetIsMontage?)))
        (return (Math|Random|RandomBoolwithWeight (Variables|Default|GetChanceToEvade)))
        (else
          (return false))))
    (:else
      (return false))))