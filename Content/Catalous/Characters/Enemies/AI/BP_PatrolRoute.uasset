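; BP_PatrolRoute is a spline-based patrol route for enemy AI that tracks a current waypoint along the Route spline.
; GetCurrentPointLocation returns the world position of the spline point at CurrentPointIndex.
; UpdatePatrolRouteLoop advances the index and wraps to the start, while UpdatePatrolRouteDirectional ping-pongs it by flipping Direction at either end.
; The route only holds patrol state and contains no movement logic.
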(fn ConstructionScript)

(fn UpdatePatrolRouteLoop
  (if (== (Variables|Default|GetCurrentPointIndex) (- (Spline|GetNumberOfSplinePoints (Variables|Default|GetRoute)) 1))
    (Variables|Default|SetCurrentPointIndex 0)
    (else
      (Math|Integer|IncrementInt (Variables|Default|GetCurrentPointIndex)))))

(fn GetCurrentPointLocation
  (return (Spline|GetLocationatSplinePoint (Variables|Default|GetRoute) (Variables|Default|GetCurrentPointIndex) "World")))

(fn UpdatePatrolRouteDirectional
  (if (== (- (Spline|GetNumberOfSplinePoints (Variables|Default|GetRoute)) 1) (Variables|Default|GetCurrentPointIndex))
    (Variables|Default|SetDirection -1)
    (elif (== (Variables|Default|GetCurrentPointIndex) 0)
      (Variables|Default|SetDirection 1)))
  (Variables|Default|SetCurrentPointIndex (+ (Variables|Default|GetCurrentPointIndex) (Variables|Default|GetDirection))))