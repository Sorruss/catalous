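; Ranged dummy enemy character that animates equipping and stowing its bow.
; EquipPrimary plays the equip or disarm montage on the mesh, chosen by the Dequip flag.
; A montage notify snaps the Primary weapon to the hand or spine socket, updates PrimaryEquiped and calls OnAttached, so the swap follows the animation.
; The construction script only calls its parent.
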(event EventBeginPlay
  (|CallParentFunction) ; This node is disabled and will not be called.\nDrag off pins to build functionality.
)

(event EventEquipPrimary
  (params (Dequip? :type Boolean))
  (bind _notifyname (Animation|Montage|PlayMontage (Variables|Character|GetMesh) (select Dequip? "/Game/Catalous/Characters/Enemies/DummyRanged/Animations/Unarmed/MDR_standing_disarm_bow_Montage.MDR_standing_disarm_bow_Montage" "/Game/Catalous/Characters/Enemies/DummyRanged/Animations/Unarmed/MDR_standing_equip_bow_Montage.MDR_standing_equip_bow_Montage"))
    (:OnNotifyBegin
      (switch name _notifyname
        (:Equip
          (Transformation|AttachComponentToComponent (Variables|Default|GetPrimary) (Variables|Character|GetMesh) (Utilities|String|SelectName "spine_bow" "hand_l_bow" Dequip?) "SnapToTarget" "SnapToTarget" "SnapToTarget" true)
          (Variables|Default|SetPrimaryEquiped? (not Dequip?))
          (Default|CallOnAttached))))))

(fn ConstructionScript
  (|CallParentFunction))