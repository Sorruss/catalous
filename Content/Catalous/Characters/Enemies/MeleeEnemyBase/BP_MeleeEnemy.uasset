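; Melee enemy Blueprint that handles sword equipping and a first combo attack, building on its parent class.
; EquipPrimary plays a draw or sheathe montage, whose notify snaps the Sword between thigh and hand sockets, updates the equipped state and fires OnAttached.
; FirstAttack plays a sword combo montage and fires OnMontageFinish on completion or interruption.
; IsPrimaryEquiped exposes the equipped state.
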(event EventBeginPlay
  (|CallParentFunction))

(event EventEquipPrimary
  (params (Dequip? :type Boolean))
  (bind _notifyname (Animation|Montage|PlayMontage (Variables|Character|GetMesh) (select Dequip? "/Game/Catalous/Characters/Enemies/MeleeEnemyBase/Animations/Idle/1HS_Idle_Combat_To_Idle_Seq_Montage.1HS_Idle_Combat_To_Idle_Seq_Montage" "/Game/Catalous/Characters/Enemies/MeleeEnemyBase/Animations/Idle/1HS_Idle_To_Idle_Combat_Seq_Montage.1HS_Idle_To_Idle_Combat_Seq_Montage"))
    (:OnNotifyBegin
      (switch name _notifyname
        (:Equip
          (Transformation|AttachComponentToComponent (Variables|Default|GetSword) (Variables|Character|GetMesh) (Utilities|String|SelectName "thigh_l_sword" "hand_r_sword" Dequip?) "SnapToTarget" "SnapToTarget" "SnapToTarget" true)
          (Variables|Default|SetPrimaryEquiped? (not Dequip?))
          (Default|CallOnAttached))))))

(event EventFirstAttack
  (Animation|Montage|PlayMontage (Variables|Character|GetMesh) "/Game/Catalous/Characters/Enemies/MeleeEnemyBase/Animations/Combo/Anim_SwordV2_Combo01_01_RM_Montage.Anim_SwordV2_Combo01_01_RM_Montage"
    (:OnCompleted
      _)
    (:OnInterrupted
      _))
  (Default|CallOnMontageFinish))

(fn ConstructionScript
  (|CallParentFunction))

(fn IsPrimaryEquiped?
  (return (Variables|Default|GetPrimaryEquiped?)))