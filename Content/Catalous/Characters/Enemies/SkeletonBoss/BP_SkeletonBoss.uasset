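; Skeleton boss enemy built from modular body and armor meshes that follow the main mesh through leader pose.
; It spawns a spear in hand, switches weapon sockets through montage notifies, dodges with random spin montages and spawns trails between weapon sockets.
; On death it strips armor, unlinks bone pieces to collapse under physics, destroys the weapon, shows the victory message, spawns a pickup and reveals the portal.
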(event EventBeginPlay
  (|CallParentFunction)
  (if (not (Variables|Default|GetDestroyedOnStart?))
    (bind _returnvalue (Game|SpawnActorfromClass "/Game/Catalous/Weapons/Melee/Spear/SkeletonSpear/BP_Weapon_Melee_SkeletonSpear.BP_Weapon_Melee_SkeletonSpear_C" (Math|Transform|MakeTransform "0, 0, 0" "0, 0, 0" "1.000000,1.000000,1.000000") "AlwaysSpawn" "MultiplyWithRoot" 0 self))
    (bind _output_get (Variables|Default|SetPrimaryWeaponActor _returnvalue))
    (Transformation|AttachComponentToComponent _output_get (Variables|Character|GetMesh) "hand_r_spear" "SnapToTarget" "SnapToTarget" "SnapToTarget" true)))

(event EventEquipPrimary
  (params (Dequip? :type Boolean))
  (Variables|Default|SetIsMontage? true)
  (bind _notifyname (Animation|Montage|PlayMontage (Variables|Character|GetMesh) (select Dequip? "/Game/Catalous/Characters/Enemies/DummyMelee/Animations/Idle/1HS_Idle_Combat_To_Idle_Seq_Montage.1HS_Idle_Combat_To_Idle_Seq_Montage" "/Game/Catalous/Characters/Enemies/DummyMelee/Animations/Idle/1HS_Idle_To_Idle_Combat_Seq_Montage.1HS_Idle_To_Idle_Combat_Seq_Montage"))
    (:OnCompleted
      (Variables|Default|SetIsMontage? false))
    (:OnNotifyBegin
      (switch name _notifyname
        (:Equip
          (Transformation|AttachComponentToComponent (Variables|Default|GetPrimaryWeaponActor) (Variables|Character|GetMesh) (Utilities|String|SelectName "thigh_l_sword" "hand_r_sword" Dequip?) "SnapToTarget" "SnapToTarget" "SnapToTarget" true)
          (Variables|Default|SetPrimaryEquiped? (not Dequip?))
          (Default|CallOnAttached))))))

(event EventFirstAttack
  (CallFunction|RandomADR -1))

(event EventEvade
  (Animation|Montage|PlayMontage (Variables|Character|GetMesh) (.OutItem (Utilities|Array|Random (Utilities|Array|MakeArray "/Game/Catalous/Characters/Enemies/SkeletonMelee/Animations/SpinDodgeLeft_Root_Montage.SpinDodgeLeft_Root_Montage" "/Game/Catalous/Characters/Enemies/SkeletonMelee/Animations/SpinDodgeRight_Root_Montage.SpinDodgeRight_Root_Montage")))))

(fn ConstructionScript
  (|CallParentFunction)
  (Components|SkinnedMesh|SetLeaderPoseComponent (Variables|Default|GetSKM_Skeleton_Lord_Body_Skull) (Variables|Character|GetMesh) false false))

(fn IsPrimaryEquiped?
  (return (Variables|Default|GetPrimaryEquiped?)))

(fn GetMeleeWeaponActor
  (return (Variables|Default|GetPrimaryWeaponActor)))

(fn SimulatePhysics
  (Components|SkinnedMesh|SetLeaderPoseComponent (Variables|Default|GetSKM_Skeleton_Lord_Body_Skull) 0 false false)
  (Physics|SetSimulatePhysics (Variables|Character|GetMesh) true))

(fn GetWeaponActor
  (|CallParentFunction)
  (return (Variables|Default|GetPrimaryWeaponActor)))

(fn OnDeathResponse
  (bind _returnvalue (Transformation|GetActorLocation))
  (|CallParentFunction)
  (Components|DestroyComponent (Variables|Default|GetSKM_Skeleton_Body_Guard))
  (CallFunction|SimulatePhysics)
  (Actor|DestroyActor (Variables|Default|GetPrimaryWeaponActor))
  (Class|BPIMCUI|ShowVictoryScreen(Message) (Game|GetPlayerCharacter 0) true (Utilities|Text|ToText(String) (Utilities|String|EnumtoString (Variables|Default|GetCharacterName))))
  (Game|SpawnActorfromClass "/Game/Catalous/Actors/Pickable/BP_Pickable_WeaponMelee.BP_Pickable_WeaponMelee_C" (Math|Transform|MakeTransform (Math|Vector|MakeVector (.x _returnvalue) (.y _returnvalue) 0.0) "0, 0, 0" "1.000000,1.000000,1.000000") "AlwaysSpawn" "MultiplyWithRoot" 0 "NewEnumerator5" "NewEnumerator3" 1 true 0)
  (bind _outactors (Actor|GetAllActorsOfClass "/Game/LevelPrototyping/Actors/Teleports/BP_Portal2.BP_Portal2_C"))
  (Rendering|SetActorHiddenInGame (Utilities|Array|Get(acopy) _outactors) false))

(fn AfterLifespanEnd
  (|CallParentFunction))

(fn StartTrail
  (params (Trail :type Niagara%20System%20Object%20Reference))
  (bind _primaryweaponactor (Variables|Default|GetPrimaryWeaponActor))
  (bind (_top _bottom) (Default|GetTrailSockets _primaryweaponactor))
  (bind _weaponmesh (Variables|/Game/Catalous/Weapons/Melee/Spear/SkeletonSpear/BP_Weapon_Melee_SkeletonSpear.BP_Weapon_Melee_SkeletonSpear_C|GetWeaponMesh _primaryweaponactor))
  (bind _returnvalue (Transformation|GetSocketLocation _weaponmesh _bottom))
  (bind _returnvalue_2 (Transformation|GetSocketLocation _weaponmesh _top))
  (bind _returnvalue_3 (Niagara|SpawnSystemAttached Trail _weaponmesh "None" (/ (+ _returnvalue_2 _returnvalue) 2.0) (Math|Rotator|MakeRotfromZ (- _returnvalue_2 _returnvalue)) "KeepWorldPosition" false))
  (Variables|Default|SetTrailSystem _returnvalue_3))

(fn EndTrail
  (bind _trailsystem (Variables|Default|GetTrailSystem)
    (:then
      (Components|DestroyComponent _trailsystem))
    (:else)))