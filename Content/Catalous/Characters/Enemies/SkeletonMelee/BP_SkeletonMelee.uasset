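; Melee skeleton enemy built from modular bone and clothing meshes that follow the main mesh through leader pose.
; On BeginPlay it spawns a red sword at the thigh socket, unless flagged destroyed on start; equip montage notifies move it between thigh and hand.
; On death it clears leader pose and ragdolls the main mesh and bone pieces so the skeleton falls apart.
; The sword is destroyed after lifespan end.
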(event EventBeginPlay
  (|CallParentFunction)
  (if (not (Variables|Default|GetDestroyedOnStart?))
    (bind _returnvalue (Game|SpawnActorfromClass "/Game/Catalous/Weapons/Melee/Swords/RedSword/BP_Weapon_Melee_RedSword.BP_Weapon_Melee_RedSword_C" (Math|Transform|MakeTransform "0, 0, 0" "0, 0, 0" "1.000000,1.000000,1.000000") "AlwaysSpawn" "MultiplyWithRoot" 0 self))
    (bind _output_get (Variables|Default|SetPrimaryWeaponActor _returnvalue))
    (Transformation|AttachComponentToComponent _output_get (Variables|Character|GetMesh) "thigh_l_sword" "SnapToTarget" "SnapToTarget" "SnapToTarget" true)))

(event EventEquipPrimary
  (params (Dequip? :type Boolean))
  (bind _notifyname (Animation|Montage|PlayMontage (Variables|Character|GetMesh) (select Dequip? "/Game/Catalous/Characters/Enemies/DummyMelee/Animations/Idle/1HS_Idle_Combat_To_Idle_Seq_Montage.1HS_Idle_Combat_To_Idle_Seq_Montage" "/Game/Catalous/Characters/Enemies/DummyMelee/Animations/Idle/1HS_Idle_To_Idle_Combat_Seq_Montage.1HS_Idle_To_Idle_Combat_Seq_Montage"))
    (:OnNotifyBegin
      (switch name _notifyname
        (:Equip
          (Transformation|AttachComponentToComponent (Variables|Default|GetPrimaryWeaponActor) (Variables|Character|GetMesh) (Utilities|String|SelectName "thigh_l_sword" "hand_r_sword" Dequip?) "SnapToTarget" "SnapToTarget" "SnapToTarget" true)
          (Variables|Default|SetPrimaryEquiped? (not Dequip?))
          (Default|CallOnAttached))))))

(event EventFirstAttack
  (CallFunction|NextADR))

(fn ConstructionScript
  (|CallParentFunction)
  (Components|SkinnedMesh|SetLeaderPoseComponent (Variables|Default|GetSKM_Skeleton_Lord_Body_Skull) (Variables|Character|GetMesh) false false))

(fn IsPrimaryEquiped?
  (return (Variables|Default|GetPrimaryEquiped?)))

(fn GetMeleeWeaponActor
  (return (Variables|Default|GetPrimaryWeaponActor)))

(fn SimulatePhysics
  (Components|SkinnedMesh|SetLeaderPoseComponent (Variables|Default|GetSKM_Skeleton_Lord_Body_Skull) 0 false false)
  (Physics|SetSimulatePhysics (Variables|Character|GetMesh) true))

(fn GetWeaponActor
  (|CallParentFunction)
  (return (Variables|Default|GetPrimaryWeaponActor)))

(fn OnDeathResponse
  (|CallParentFunction)
  (CallFunction|SimulatePhysics))

(fn AfterLifespanEnd
  (|CallParentFunction)
  (Actor|DestroyActor (Variables|Default|GetPrimaryWeaponActor)))