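; Ranged skeleton enemy that fights with a bow and a short sword, dropping an ammo pickup on death.
; Spawns both weapons at BeginPlay and swaps them between holster and hand sockets on equip montage notifies.
; Attacks either fire toward the AI controller's target via the bow mechanics component or play a sword montage, then signal completion.
; Modular body meshes follow the main mesh's pose until death unlinks them and bones simulate physics.
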(event Custom|DequipPrimaryNoAnimation
  (Transformation|AttachComponentToComponent (Variables|/Game/Catalous/Weapons/Ranged/Bows/DefaultBow/BP_Weapon_Ranged_DefaultBow.BP_Weapon_Ranged_DefaultBow_C|GetWeaponSkeletal (Variables|Default|GetPrimaryActor)) (Variables|Character|GetMesh) "spine_bow" "SnapToTarget" "SnapToTarget" "SnapToTarget" true)
  (Variables|Default|SetPrimaryEquiped? false)
  (Variables|/Game/Catalous/Components/AC_BowMechanics_AI.AC_BowMechanics_AI_C|SetIsAiming? (Variables|Default|GetAC_BowMechanics_AI) false))

(event Custom|DequipSecondaryNoAnimation
  (Transformation|AttachComponentToComponent (Variables|Default|GetSecondaryActor) (Variables|Character|GetMesh) "thigh_l_dagger" "SnapToTarget" "SnapToTarget" "SnapToTarget" true)
  (Variables|Default|SetSecondaryEquipped? false))

(event Custom|FirePrimary
  (bind _ac_bowmechanics_ai (Variables|Default|GetAC_BowMechanics_AI))
  (Default|AimBegin _ac_bowmechanics_ai)
  (Default|StartDrawing _ac_bowmechanics_ai)
  (Utilities|FlowControl|Delay (Math|Random|RandomFloatinRange 0.7 1.0))
  (bind _aicontroller_0 (Variables|Default|GetAIController_0)
    (:then
      (bind _direction (Default|GetDirectiontoTarget _aicontroller_0))
      (Default|FireBegin _ac_bowmechanics_ai _direction)
      (Utilities|FlowControl|Delay 1.0)
      (Default|CallOnMontageFinish 0.0))
    (:else)))

(event Custom|FireSecondary
  (Animation|Montage|PlayMontage (Variables|Character|GetMesh) "/Game/Catalous/Characters/Enemies/DummyMelee/Animations/Combo/Anim_SwordV2_Combo01_01_RM_Montage.Anim_SwordV2_Combo01_01_RM_Montage"
    (:OnCompleted
      (Default|CallOnMontageFinish 0.5))))

(event EventBeginPlay
  (|CallParentFunction)
  (if (not (Variables|Default|GetDestroyedOnStart?))
    (bind _returnvalue (Game|SpawnActorfromClass "/Game/Catalous/Weapons/Ranged/Bows/DefaultBow/BP_Weapon_Ranged_DefaultBow.BP_Weapon_Ranged_DefaultBow_C" (Math|Transform|MakeTransform "0, 0, 0" "0, 0, 0" "1.000000,1.000000,1.000000") "AlwaysSpawn" "MultiplyWithRoot" 0 self))
    (bind _output_get (Variables|Default|SetPrimaryActor _returnvalue))
    (Transformation|AttachComponentToComponent (Variables|/Game/Catalous/Weapons/Ranged/Bows/DefaultBow/BP_Weapon_Ranged_DefaultBow.BP_Weapon_Ranged_DefaultBow_C|GetWeaponSkeletal _output_get) (Variables|Character|GetMesh) "spine_bow" "SnapToTarget" "SnapToTarget" "SnapToTarget" true)
    (bind _asaic_enemy_base (Utilities|Casting|CastToAIC_Enemy_Base (AI|GetAIController self)))
    (Variables|Default|SetAIController_0 _asaic_enemy_base)
    (bind _returnvalue_2 (Game|SpawnActorfromClass "/Game/Catalous/Weapons/Melee/Swords/ShortSword/BP_Weapon_Melee_ShortSword.BP_Weapon_Melee_ShortSword_C" (Math|Transform|MakeTransform "0, 0, 0" "0, 0, 0" "1.000000,1.000000,1.000000") "AlwaysSpawn" "MultiplyWithRoot" 0 self))
    (bind _output_get_2 (Variables|Default|SetSecondaryActor _returnvalue_2))
    (Transformation|AttachComponentToComponent _output_get_2 (Variables|Character|GetMesh) "thigh_l_dagger" "SnapToTarget" "SnapToTarget" "SnapToTarget" true)))

(event EventEquipPrimary
  (params (Dequip? :type Boolean))
  (if (Variables|Default|GetSecondaryEquipped?)
    (CallFunction|DequipSecondaryNoAnimation))
  (bind _notifyname (Animation|Montage|PlayMontage (Variables|Character|GetMesh) (select Dequip? "/Game/Catalous/Characters/Enemies/DummyRanged/Animations/Unarmed/MDR_standing_disarm_bow_Montage.MDR_standing_disarm_bow_Montage" "/Game/Catalous/Characters/Enemies/DummyRanged/Animations/Unarmed/MDR_standing_equip_bow_Montage.MDR_standing_equip_bow_Montage"))
    (:OnNotifyBegin
      (switch name _notifyname
        (:Equip
          (Transformation|AttachComponentToComponent (Variables|/Game/Catalous/Weapons/Ranged/Bows/DefaultBow/BP_Weapon_Ranged_DefaultBow.BP_Weapon_Ranged_DefaultBow_C|GetWeaponSkeletal (Variables|Default|GetPrimaryActor)) (Variables|Character|GetMesh) (Utilities|String|SelectName "spine_bow" "hand_l_bow" Dequip?) "SnapToTarget" "SnapToTarget" "SnapToTarget" true)
          (Variables|Default|SetPrimaryEquiped? (not Dequip?))
          (Default|CallOnAttached))))))

(event EventFirstAttack
  (if (Variables|Default|GetPrimaryEquiped?)
    (CallFunction|FirePrimary)
    (else
      (CallFunction|FireSecondary))))

(event EventReloadWeapon
  (Animation|Montage|PlayMontage (Variables|Character|GetMesh) "/Game/Catalous/Characters/Enemies/DummyRanged/Animations/Combat/MDR_standing_draw_arrow_Montage.MDR_standing_draw_arrow_Montage"
    (:then
      (Variables|/Game/Catalous/Components/AC_BowMechanics_AI.AC_BowMechanics_AI_C|SetIsAiming? (Variables|Default|GetAC_BowMechanics_AI) true))
    (:OnCompleted
      (Default|CallOnMontageFinish 0.0 :!label _label))
    (:OnInterrupted
      (goto _label))))

(event EventEquipSecondary
  (params (Dequip? :type Boolean))
  (if (Variables|Default|GetPrimaryEquiped?)
    (CallFunction|DequipPrimaryNoAnimation))
  (bind _notifyname (Animation|Montage|PlayMontage (Variables|Character|GetMesh) (select Dequip? "/Game/Catalous/Characters/Enemies/DummyMelee/Animations/Idle/1HS_Idle_Combat_To_Idle_Seq_Montage.1HS_Idle_Combat_To_Idle_Seq_Montage" "/Game/Catalous/Characters/Enemies/DummyMelee/Animations/Idle/1HS_Idle_To_Idle_Combat_Seq_Montage.1HS_Idle_To_Idle_Combat_Seq_Montage"))
    (:OnNotifyBegin
      (switch name _notifyname
        (:equip
          (Transformation|AttachComponentToComponent (Variables|Default|GetSecondaryActor) (Variables|Character|GetMesh) (Utilities|String|SelectName "thigh_l_dagger" "hand_r_dagger" Dequip?) "SnapToTarget" "SnapToTarget" "SnapToTarget" true)
          (Variables|Default|SetSecondaryEquipped? (not Dequip?))
          (Default|CallOnAttached))))))

(fn ConstructionScript
  (|CallParentFunction)
  (Components|SkinnedMesh|SetLeaderPoseComponent (Variables|Default|GetSKM_Skeleton_Lord_Body_Skull) (Variables|Character|GetMesh) false false))

(fn GetPrimaryasRanged
  (return (Variables|Default|GetPrimaryActor)))

(fn GetMeleeWeaponActor
  (return (Variables|Default|GetSecondaryActor)))

(fn OnAbortRealodWeapon
  (|CallParentFunction)
  (Variables|/Game/Catalous/Components/AC_BowMechanics_AI.AC_BowMechanics_AI_C|SetIsAiming? (Variables|Default|GetAC_BowMechanics_AI) false))

(fn SimulatePhysics
  (Components|SkinnedMesh|SetLeaderPoseComponent (Variables|Default|GetSKM_Skeleton_Lord_Body_Skull) 0 false false)
  (Physics|SetSimulatePhysics (Variables|Character|GetMesh) true))

(fn GetWeaponActor
  (|CallParentFunction)
  (return (Variables|Default|GetSecondaryActor)))

(fn OnDeathResponse
  (bind _returnvalue (Transformation|GetActorLocation))
  (|CallParentFunction)
  (Game|SpawnActorfromClass "/Game/Catalous/Actors/Pickable/BP_Pickable_Ammo.BP_Pickable_Ammo_C" (Math|Transform|MakeTransform (Math|Vector|MakeVector (.x _returnvalue) (.y _returnvalue) 0.0) "0, 0, 0" "1.000000,1.000000,1.000000") "AlwaysSpawn" "MultiplyWithRoot" 0 "NewEnumerator0" "NewEnumerator1" 5 true 0)
  (CallFunction|SimulatePhysics))

(fn AfterLifespanEnd
  (|CallParentFunction)
  (Actor|DestroyActor (Variables|Default|GetPrimaryActor))
  (Actor|DestroyActor (Variables|Default|GetSecondaryActor)))