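; Walking dummy enemy that can draw and sheathe a one-handed sword.
; EquipPrimary plays the matching idle-to-combat or combat-to-idle montage, whose notify snaps the sword between the thigh and right-hand sockets.
; Montage completion or interruption both fire the montage-finish call and update the equipped flag, which IsPrimaryEquiped exposes.
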(event EventBeginPlay
  (|CallParentFunction))

(event EventEquipPrimary
  (params (Dequip? :type Boolean))
  (bind _notifyname (Animation|Montage|PlayMontage (Variables|Character|GetMesh) (select Dequip? "/Game/Catalous/Characters/Enemies/WalkingDummy/Animations/Idle/1HS_Idle_Combat_To_Idle_Seq_Montage.1HS_Idle_Combat_To_Idle_Seq_Montage" "/Game/Catalous/Characters/Enemies/WalkingDummy/Animations/Idle/1HS_Idle_To_Idle_Combat_Seq_Montage.1HS_Idle_To_Idle_Combat_Seq_Montage"))
    (:OnCompleted
      (Default|CallOnMontageFinish :!label _label)
      (Variables|Default|SetPrimaryEquiped? (not Dequip?)))
    (:OnInterrupted
      (goto _label))
    (:OnNotifyBegin
      (switch name _notifyname
        (:Equip
          (Transformation|AttachComponentToComponent (Variables|Default|GetSword) (Variables|Character|GetMesh) (Utilities|String|SelectName "thigh_l_sword" "hand_r_sword" Dequip?) "SnapToTarget" "SnapToTarget" "SnapToTarget" true))))))

(fn ConstructionScript
  (|CallParentFunction))

(fn IsPrimaryEquiped?
  (return (Variables|Default|GetPrimaryEquiped?)))