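; Attack component for BP_Knight that handles melee combos and the equipping and stowing of swords and greatswords.
; Attack picks light or heavy montages from the Ctrl state, then dispatches by weapon type: fists and greatsword spend stamina to attack, while sword only equips.
; Combos reset at the last montage or via a retriggerable delay, and notifies release the animation lock or swap weapon sockets.
; A macro switches blendspaces immediately on equip and at montage blend-out on dequip.
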(event Custom|EquipSword
  (params (Dequip? :type Boolean))
  (bind _bp_knight (Variables|Default|GetBP%20Knight))
  (bind _bp_knight_2 (Variables|Default|GetBP%20Knight))
  (Animation|Montage|PlayMontage (Variables|/Script/Engine.Character|GetMesh _bp_knight_2) "/Game/Catalous/Characters/MC/GothicKnight/Animation/Sword/Equip/Equip_Sword_Montage.Equip_Sword_Montage"
    (:then
      (Utilities|FirstMontageorBS Dequip? :!label _label
        (:execute
          (Default|UpdateBS (Variables|/Game/Catalous/Characters/MC/BP_Knight.BP_Knight_C|GetAnimInstance _bp_knight_2) (select Dequip? "NewEnumerator1" "NewEnumerator2")))))
    (:OnBlendOut
      (goto _label FirstMontage))
    (:OnNotifyBegin
      (Transformation|AttachComponentToComponent (Variables|/Game/Catalous/Characters/MC/BP_Knight.BP_Knight_C|GetPrimaryWeapon _bp_knight) (Variables|/Script/Engine.Character|GetMesh _bp_knight) (Utilities|String|SelectName "sword_unarmed" "hand_r_sword" Dequip?) "SnapToTarget" "SnapToTarget" "SnapToTarget" true))))

(event Custom|EquipGreatsword
  (params (Dequip? :type Boolean))
  (bind _bp_knight (Variables|Default|GetBP%20Knight))
  (bind _bp_knight_2 (Variables|Default|GetBP%20Knight))
  (Animation|Montage|PlayMontage (Variables|/Script/Engine.Character|GetMesh _bp_knight) (select Dequip? "/Game/Catalous/Characters/MC/GothicKnight/Animation/Greatsword/Idle/GreatSword_Unarm_Montage.GreatSword_Unarm_Montage" "/Game/Catalous/Characters/MC/GothicKnight/Animation/Greatsword/Idle/GreatSword_Equip_Montage.GreatSword_Equip_Montage")
    (:then
      (Utilities|FirstMontageorBS Dequip? :!label _label
        (:execute
          (Default|UpdateBS (Variables|/Game/Catalous/Characters/MC/BP_Knight.BP_Knight_C|GetAnimInstance _bp_knight) (select Dequip? "NewEnumerator1" "NewEnumerator3")))))
    (:OnBlendOut
      (goto _label FirstMontage))
    (:OnNotifyBegin
      (Transformation|AttachComponentToComponent (Variables|/Game/Catalous/Characters/MC/BP_Knight.BP_Knight_C|GetPrimaryWeapon _bp_knight_2) (Variables|/Script/Engine.Character|GetMesh _bp_knight_2) (Utilities|String|SelectName "back_greatsword" "hand_r_greatsword" Dequip?) "SnapToTarget" "SnapToTarget" "SnapToTarget" true))))

(event Custom|DequipPrimaryWeapon
  (Variables|Default|SetIsWeaponEquiped? false)
  (switch Utilities|FlowControl|Switch|SwitchonE_WeaponSubtype (Variables|Default|GetType)
    (:NewEnumerator2
      (CallFunction|EquipSword true))
    (:NewEnumerator3
      (CallFunction|EquipGreatsword true))))

(event Custom|UpdateCombo
  (bind _result (Math|Integer|IncrementInt (Variables|Default|GetComboCounter))
    (:%20%20
      (if (== _result (Variables|Default|GetMaxCombo))
        _
        (else
          (Utilities|FlowControl|RetriggerableDelay 2.0)))
      (Variables|Default|SetComboCounter 0))))

(event Custom|PerformAttack
  (Variables|Default|SetInAnimationLock? true)
  (bind _notifyname (Animation|Montage|PlayMontage (Variables|/Script/Engine.Character|GetMesh (Variables|Default|GetBP%20Knight)) (Utilities|Array|Get(acopy) (Variables|Default|GetAttacks%20Montages) (Variables|Default|GetComboCounter)))
    (:then
      (Variables|Default|SetCanDequip? false))
    (:OnCompleted
      (Variables|Default|SetCanDequip? true))
    (:OnNotifyBegin
      (if (== _notifyname "DropAnimationLock")
        (Variables|Default|SetInAnimationLock? false)))))

(event EventBeginPlay
  (bind _asbp_knight (Utilities|Casting|CastToBP_Knight (Components|GetOwner)))
  (Variables|Default|SetBP%20Knight _asbp_knight))

(fn Attack
  (params (Weapon :type S%20Weapon%20Melee%20Structure))
  (bind _output_get (Variables|Default|SetWeapon Weapon))
  (Variables|Default|SetType (.Subtype (Utilities|Struct|BreakS_WeaponBase (Utilities|Struct|BreakS_WeaponMelee _output_get))))
  (CallFunction|DefineAttackType)
  (bind _output_get_2 (Variables|Default|SetAttacks%20Montages (Utilities|Select :Index (Variables|Default|GetAttackType) :NewEnumerator0 0 :NewEnumerator1 (.LightAttacks (Utilities|Struct|BreakS_AttacksMontages (.AttacksMontages (Utilities|Struct|BreakS_WeaponBase (Utilities|Struct|BreakS_WeaponMelee _output_get))))) :NewEnumerator2 (.HeavyAttacks (Utilities|Struct|BreakS_AttacksMontages (.AttacksMontages (Utilities|Struct|BreakS_WeaponBase (Utilities|Struct|BreakS_WeaponMelee _output_get))))) :NewEnumerator3 (Utilities|Array|MakeArray (.DodgeAttack (Utilities|Struct|BreakS_AttacksMontages (.AttacksMontages (Utilities|Struct|BreakS_WeaponBase (Utilities|Struct|BreakS_WeaponMelee _output_get)))))))))
  (Variables|Default|SetMaxCombo (Utilities|Array|Length _output_get_2))
  (switch Utilities|FlowControl|Switch|SwitchonE_WeaponSubtype (Variables|Default|GetType)
    (:NewEnumerator1
      (CallFunction|AttackFists))
    (:NewEnumerator2
      (CallFunction|AttackSword))
    (:NewEnumerator3
      (CallFunction|AttackGreatsword))))

(fn AttackFists
  (bind _weapon (Variables|Default|GetWeapon))
  (bind _bp_knight (Variables|Default|GetBP%20Knight))
  (bind _weaponbase (Utilities|Struct|BreakS_WeaponMelee _weapon))
  (bind _staminacost (Utilities|Struct|BreakS_WeaponBase _weaponbase))
  (if (Default|CanAffordAmount? (Variables|/Game/Catalous/Characters/MC/BP_Knight.BP_Knight_C|GetAC_Stamina (Variables|Default|GetBP%20Knight)) _staminacost)
    (Default|UseStaminaAttack (Variables|/Game/Catalous/Characters/MC/BP_Knight.BP_Knight_C|GetAC_Stamina _bp_knight) _staminacost)
    (Default|StandStill _bp_knight true)
    (CallFunction|PerformAttack)
    (CallFunction|UpdateCombo)))

(fn AttackSword
  (if (not (Variables|Default|GetIsWeaponEquiped?))
    (CallFunction|EquipSword false)
    (Variables|Default|SetIsWeaponEquiped? true)))

(fn AttackGreatsword
  (bind _weapon (Variables|Default|GetWeapon))
  (bind _bp_knight (Variables|Default|GetBP%20Knight))
  (bind _weaponbase (Utilities|Struct|BreakS_WeaponMelee _weapon))
  (bind _staminacost (Utilities|Struct|BreakS_WeaponBase _weaponbase))
  (if (not (Variables|Default|GetIsWeaponEquiped?))
    (CallFunction|EquipGreatsword false)
    (Variables|Default|SetIsWeaponEquiped? true)
    (else
      (if (Utilities|Enum|Equal(Enum) (Variables|Default|GetAttackType) "NewEnumerator2")
        _
        (else
          _))
      (if (Default|CanAffordAmount? (Variables|/Game/Catalous/Characters/MC/BP_Knight.BP_Knight_C|GetAC_Stamina (Variables|Default|GetBP%20Knight)) _staminacost)
        (Default|UseStaminaAttack (Variables|/Game/Catalous/Characters/MC/BP_Knight.BP_Knight_C|GetAC_Stamina _bp_knight) _staminacost)
        (Default|StandStill _bp_knight true)
        (CallFunction|PerformAttack)
        (CallFunction|UpdateCombo)))))

(fn DefineAttackType
  (if (Variables|/Game/Catalous/Characters/MC/BP_Knight.BP_Knight_C|GetIsPressingCtrl? (Variables|Default|GetBP%20Knight))
    (Variables|Default|SetAttackType "NewEnumerator2")
    (else
      (Variables|Default|SetAttackType "NewEnumerator1"))))