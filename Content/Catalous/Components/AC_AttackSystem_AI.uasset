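; Attack component for BP_Generic_Enemy that detects and reports hits from unarmed and weapon attacks.
; Looping timers sweep spheres along a chosen body-part socket, or line traces along weapon socket paths, cross-linking neighbouring sockets to cover gaps.
; Each newly hit actor gets a damage message and a reported damage event.
; Melee messages carry weapon physical damage, parry, block and interrupt flags, and a dot-product-derived hit direction.
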(event Custom|Start%20Melee%20Damage%20Trace
  ;[0.15 0.15 0.15 0.5] Weapon Traces: Melee
  (CallFunction|UpdateWeaponSockets)
  (bind _returnvalue (Utilities|Time|SetTimerbyEvent (delegate Custom|Damage%20Melee%20Trace) (Variables|Default|GetTracingEveryNTime) true)))

(event Custom|StartCloseCombatTrace
  (params (BodyPart :type E_BodyParts%20Enum :default "NewEnumerator0"))
  ;[0.15 0.15 0.15 0.5] Weapon Traces: Close Combat
  (Variables|Default|SetLastDamageTraceLocationCC (Transformation|GetSocketLocation (Variables|/Script/Engine.Character|GetMesh (Variables|Default|GetBP%20Enemy)) (Utilities|Select :Index BodyPart :NewEnumerator0 "None" :NewEnumerator1 "head" :NewEnumerator2 "hand_l" :NewEnumerator3 "spine_03" :NewEnumerator4 "hand_r" :NewEnumerator5 "foot_l" :NewEnumerator6 "foot_r")))
  (Utilities|Array|Clear (Variables|Default|GetAlreadyHittedActors))
  (bind _returnvalue (Utilities|Time|SetTimerbyEvent (delegate Custom|DamageCloseCombatTrace) 0.05 true)))

(event Custom|End%20Melee%20Damage%20Trace
  ;[0.15 0.15 0.15 0.5] Weapon Traces: Melee
  (if true
    (Utilities|Time|ClearandInvalidateTimerbyHandle (stale Custom|Start%20Melee%20Damage%20Trace _returnvalue))
    (Utilities|Array|Clear (Variables|Default|GetAlreadyHittedActors))))

(event Custom|EndCloseCombatTrace
  ;[0.15 0.15 0.15 0.5] Weapon Traces: Close Combat
  (if (Utilities|Time|IsValidTimerHandle (stale Custom|StartCloseCombatTrace _returnvalue))
    (Utilities|Time|ClearandInvalidateTimerbyHandle (stale Custom|StartCloseCombatTrace _returnvalue))))

(event Custom|DamageCloseCombatTrace
  ;[0.15 0.15 0.15 0.5] Weapon Traces: Close Combat
  (bind (_outhits _returnvalue) (Collision|MultiSphereTraceByChannel (Variables|Default|GetLastDamageTraceLocationCC) (Transformation|GetSocketLocation (Variables|/Script/Engine.Character|GetMesh (Variables|Default|GetBP%20Enemy)) (Utilities|Select :Index (stale Custom|StartCloseCombatTrace BodyPart) :NewEnumerator0 "None" :NewEnumerator1 "head" :NewEnumerator2 "hand_l" :NewEnumerator3 "spine_03" :NewEnumerator4 "hand_r" :NewEnumerator5 "foot_l" :NewEnumerator6 "foot_r")) 3e+01 "TraceTypeQuery3" false 0 "None"))
  (Variables|Default|SetLastDamageTraceLocationCC (Transformation|GetSocketLocation (Variables|/Script/Engine.Character|GetMesh (Variables|Default|GetBP%20Enemy)) (Utilities|Select :Index (stale Custom|StartCloseCombatTrace BodyPart) :NewEnumerator0 "None" :NewEnumerator1 "head" :NewEnumerator2 "hand_l" :NewEnumerator3 "spine_03" :NewEnumerator4 "hand_r" :NewEnumerator5 "foot_l" :NewEnumerator6 "foot_r")))
  (if _returnvalue
    (for _array_element _outhits
      (if (not (Utilities|Array|ContainsItem (Variables|Default|GetAlreadyHittedActors) (.HitActor (Collision|BreakHitResult _array_element))))
        (Utilities|Array|Add (Variables|Default|GetAlreadyHittedActors) (.HitActor (Collision|BreakHitResult _array_element)))
        (Class|BPIDamagable|GetDamaged(Message) (.HitActor (Collision|BreakHitResult _array_element)))
        (Class|AISenseDamage|ReportDamageEvent (.HitActor (Collision|BreakHitResult _array_element)) 0 (Utilities|BodyPart2Damage (stale Custom|StartCloseCombatTrace BodyPart)) (Transformation|GetActorLocation (Variables|Default|GetBP%20Enemy)) "0, 0, 0" "None")))))

(event Custom|Damage%20Melee%20Trace
  (bind _weaponsocketlastlocation (Variables|Default|GetWeaponSocketLastLocation))
  (bind _bp_enemy (Variables|Default|GetBP%20Enemy))
  (bind _bp_enemy_2 (Variables|Default|GetBP%20Enemy))
  (bind _weaponactor (Variables|Default|GetWeaponActor))
  (bind _weaponsocketlastlastlocation (Variables|Default|GetWeaponSocketLastLastLocation))
  (bind _data (Default|GetWeaponBaseData _weaponactor))
  (bind _array (Utilities|Array|MakeArray _bp_enemy))
  (bind _attackpower (Utilities|Struct|BreakS_WeaponBase _data))
  (bind _physical (Utilities|Struct|BreakS_AttackPower _attackpower))
  ;[0.15 0.15 0.15 0.5] Weapon Traces: Melee
  (bind _keys (Utilities|Map|Keys _weaponsocketlastlocation))
  (for (_array_element _array_index) _keys
    (Variables|Default|SetIsThisFirstSocket? (== 0 _array_index))
    (bind (_outhits _returnvalue) (Collision|MultiLineTraceByChannel (.Value (Utilities|Map|Find _weaponsocketlastlocation _array_element)) (Transformation|GetSocketLocation (Default|GetMesh (Variables|Default|GetWeaponActor)) _array_element) "TraceTypeQuery3" false _array (Variables|Default|GetDrawDebugTraces?)))
    (Variables|Default|SetHittedActorsFirstTrace _outhits)
    (if (Variables|Default|GetIsThisFirstSocket?)
      _
      (else
        (bind _keys_2 (Utilities|Map|Keys _weaponsocketlastlastlocation))
        (bind (_outhits_2 _returnvalue_2) (Collision|MultiLineTraceByChannel (.Value (Utilities|Map|Find _weaponsocketlastlastlocation (Utilities|Array|Get(acopy) _keys_2 (- _array_index 1)))) (.Value (Utilities|Map|Find _weaponsocketlastlocation _array_element)) "TraceTypeQuery3" false _array (Variables|Default|GetDrawDebugTraces?)))
        (Variables|Default|SetHittedActorsSecondTrace _outhits_2)
        (Utilities|Map|Add (Variables|Default|GetWeaponSocketLastLastLocation) (Utilities|Array|Get(acopy) _keys_2 (- _array_index 1)) (.Value (Utilities|Map|Find (Variables|Default|GetWeaponSocketLastLocation) (Utilities|Array|Get(acopy) _keys_2 (- _array_index 1)))))))
    (Utilities|Map|Add (Variables|Default|GetWeaponSocketLastLocation) _array_element (Transformation|GetSocketLocation (Default|GetMesh (Variables|Default|GetWeaponActor)) _array_element))
    (if (or _returnvalue _returnvalue_2)
      (Utilities|Array|AppendArray (Variables|Default|GetHittedActorsFirstTrace) (Variables|Default|GetHittedActorsSecondTrace))
      (for _array_element_2 (Variables|Default|GetHittedActorsFirstTrace)
        (if (not (Utilities|Array|ContainsItem (Variables|Default|GetAlreadyHittedActors) (.HitActor (Collision|BreakHitResult _array_element_2))))
          (Utilities|Array|Add (Variables|Default|GetAlreadyHittedActors) (.HitActor (Collision|BreakHitResult _array_element_2)))
          (bind _damagedactorstate (Class|BPIDamagable|GetDamagedActorState(Message) (.HitActor (Collision|BreakHitResult _array_element_2))))
          (Class|BPIDamagable|GetDamaged(Message) (.HitActor (Collision|BreakHitResult _array_element_2)) (Utilities|Struct|MakeS_DamageInfo (Variables|Default|GetBP%20Enemy) _physical true true true false (CallFunction|GetDirectionOfAnotherActor (.HitActor (Collision|BreakHitResult _array_element_2)) (Variables|Default|GetBP%20Enemy)) _damagedactorstate))
          (Class|AISenseDamage|ReportDamageEvent (.HitActor (Collision|BreakHitResult _array_element_2)) _bp_enemy_2 _physical (Transformation|GetActorLocation _bp_enemy_2) "0, 0, 0" "None"))))))

(event EventBeginPlay
  (bind _asbp_generic_enemy (Utilities|Casting|CastToBP_Generic_Enemy (Components|GetOwner)))
  (Variables|Default|SetBP%20Enemy _asbp_generic_enemy))

(fn UpdateWeaponSockets
  (bind _actor (Default|GetWeaponActor (Variables|Default|GetBP%20Enemy)))
  (bind _output_get (Variables|Default|SetWeaponActor _actor))
  (for _array_element (Variables|/Game/Catalous/Weapons/BP_Generic_Weapon.BP_Generic_Weapon_C|GetSockets _output_get)
    (Utilities|Map|Add (Variables|Default|GetWeaponSocketLastLocation) _array_element (Transformation|GetSocketLocation (Default|GetMesh _output_get) _array_element))
    (Utilities|Map|Add (Variables|Default|GetWeaponSocketLastLastLocation) _array_element (Transformation|GetSocketLocation (Default|GetMesh _output_get) _array_element))))

(fn GetDirectionOfAnotherActor
  (params (TargetActor :type Actor%20Object%20Reference) (AnotherActor :type Actor%20Object%20Reference))
  (bind _returnvalue (Transformation|GetActorForwardVector AnotherActor))
  (bind _returnvalue_2 (Transformation|GetActorForwardVector TargetActor))
  (bind _returnvalue_3 (Transformation|GetActorLocation AnotherActor))
  (bind _returnvalue_4 (Transformation|GetActorLocation TargetActor))
  (bind _returnvalue_5 (Transformation|GetActorRightVector TargetActor))
  (bind _returnvalue_6 (Math|Vector|Normalize _returnvalue))
  (bind _returnvalue_7 (Math|Vector|Normalize _returnvalue_2))
  (bind _returnvalue_8 (- _returnvalue_4 _returnvalue_3))
  (bind _returnvalue_9 (Math|Vector|DotProduct _returnvalue_7 _returnvalue_6))
  (bind _returnvalue_10 (Math|Vector|DotProduct _returnvalue_8 _returnvalue_5))
  (if (>= _returnvalue_9 0.6)
    (LocalVariables|SetReturnValueDirection "NewEnumerator1")
    (elif (<= _returnvalue_9 -0.8)
      (LocalVariables|SetReturnValueDirection "NewEnumerator6")
      (elif (> _returnvalue_10 0.0)
        (LocalVariables|SetReturnValueDirection "NewEnumerator3")
        (elif (< _returnvalue_10 0.0)
          (LocalVariables|SetReturnValueDirection "NewEnumerator2")
          (else
            (LocalVariables|SetReturnValueDirection "NewEnumerator1"))))))
  (return (LocalVariables|GetReturnValueDirection)))