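; Actor component for BP_Knight that runs blocking by active weapon type, plus hit reactions, block breaks and a parry flag.
; Fists and melee weapons play montages from weapon block data and change movement mode, with melee weapons also swapping between block and equip sockets.
; Bow block instead starts aiming through the bow mechanics component after stamina and ammo checks.
; Hit reactions resume blocking on blend out, while breaks lock animation until their montage completes.
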(event Custom|BlockEndMeleeType
  (bind _character (Variables|Default|GetCharacter))
  (bind _character_2 (Variables|Default|GetCharacter))
  (bind _currentblockdata (Variables|Default|GetCurrentBlockData))
  (bind _weapon (Default|GetWeaponActor _character))
  (bind _mesh (Variables|/Script/Engine.Character|GetMesh _character_2))
  ;[0.15 0.15 0.15 0.5] Melee Type
  (Transformation|AttachComponentToComponent _weapon _mesh (Utilities|Struct|BreakS_Equip_Dequip (Variables|/Game/Catalous/Weapons/BP_Generic_Weapon.BP_Generic_Weapon_C|GetEquipDequip _weapon)) "SnapToTarget" "SnapToTarget" "SnapToTarget" true)
  (Animation|Montage|PlayMontage _mesh (.fullmontage _currentblockdata) 1.0 0.0 (.loopendsectionname _currentblockdata)))

(event Custom|BlockStartFists
  (params (BlockData :type S%20Weapon%20Block%20Structure))
  ;[0.15 0.15 0.15 0.5] Fists Type
  (Animation|Montage|PlayMontage (Variables|/Script/Engine.Character|GetMesh (Variables|Default|GetCharacter)) (.fullmontage BlockData)))

(event Custom|BlockStartMeleeType
  (params (BlockData :type S%20Weapon%20Block%20Structure))
  (bind _character (Variables|Default|GetCharacter))
  (bind _character_2 (Variables|Default|GetCharacter))
  (bind _weapon (Default|GetWeaponActor _character_2))
  (bind _mesh (Variables|/Script/Engine.Character|GetMesh _character))
  (bind _equipdequip (Variables|/Game/Catalous/Weapons/BP_Generic_Weapon.BP_Generic_Weapon_C|GetEquipDequip _weapon))
  (bind (_slot_equip _slot_block) (Utilities|Struct|BreakS_Equip_Dequip _equipdequip))
  ;[0.15 0.15 0.15 0.5] Melee Type
  (Transformation|AttachComponentToComponent _weapon _mesh _slot_block "SnapToTarget" "SnapToTarget" "SnapToTarget" true)
  (Animation|Montage|PlayMontage _mesh (.fullmontage BlockData)
    (:OnInterrupted
      (Transformation|AttachComponentToComponent _weapon _mesh _slot_equip "SnapToTarget" "SnapToTarget" "SnapToTarget" true))))

(event Custom|BlockHitReaction
  (bind _character (Variables|Default|GetCharacter))
  (bind _currentblockdata (Variables|Default|GetCurrentBlockData))
  (bind _character_2 (Variables|Default|GetCharacter))
  (bind _hitreaction (Utilities|Struct|BreakS_WeaponBlock _currentblockdata))
  (bind _weapon (Default|GetWeaponActor _character_2))
  (bind _mesh (Variables|/Script/Engine.Character|GetMesh _character))
  ;[0.15 0.15 0.15 0.5] Block Hit Reaction
  (if (and (Variables|Default|GetIsBlocking?) (not (Variables|Default|GetBlockBroken?)))
    (switch Utilities|FlowControl|Switch|SwitchonE_WeaponSubtype (Default|GetActiveWeaponType (Variables|Default|GetCharacter))
      (:NewEnumerator0
        (Animation|Montage|PlayMontage _mesh _hitreaction :!label _label
          (:OnBlendOut
            (if (Variables|Default|GetIsBlocking?)
              (CallFunction|BlockStartFists (Variables|Default|GetCurrentBlockData))))))
      (:NewEnumerator1
        (goto _label))
      (:NewEnumerator2
        (Animation|Montage|PlayMontage _mesh _hitreaction :!label _label_2
          (:then
            (Transformation|AttachComponentToComponent _weapon _mesh (Utilities|Struct|BreakS_Equip_Dequip (Variables|/Game/Catalous/Weapons/BP_Generic_Weapon.BP_Generic_Weapon_C|GetEquipDequip _weapon)) "SnapToTarget" "SnapToTarget" "SnapToTarget" true))
          (:OnBlendOut
            (if (Variables|Default|GetIsBlocking?)
              (CallFunction|BlockStartMeleeType (Variables|Default|GetCurrentBlockData))))))
      (:NewEnumerator3
        (goto _label_2)))))

(event Custom|BlockEndFists
  (bind _currentblockdata (Variables|Default|GetCurrentBlockData))
  ;[0.15 0.15 0.15 0.5] Fists Type
  (Animation|Montage|PlayMontage (Variables|/Script/Engine.Character|GetMesh (Variables|Default|GetCharacter)) (.fullmontage _currentblockdata) 1.0 0.0 (.loopendsectionname _currentblockdata)))

(event Custom|BlockBreak
  (bind _character (Variables|Default|GetCharacter))
  (bind _character_2 (Variables|Default|GetCharacter))
  ;[0.15 0.15 0.15 0.5] Block Break Reaction
  (Variables|Default|SetBlockBroken? true)
  (CallFunction|BlockEnd)
  (Default|AnimationLock _character true)
  (Variables|/Game/Catalous/Characters/MC/BP_Knight.BP_Knight_C|SetCanRoll? _character false)
  (Animation|Montage|PlayMontage (Variables|/Script/Engine.Character|GetMesh (Variables|Default|GetCharacter)) (Utilities|Struct|BreakS_WeaponBlock (Variables|Default|GetCurrentBlockData))
    (:OnCompleted
      (Default|AnimationLock _character_2 false)
      (Variables|/Game/Catalous/Characters/MC/BP_Knight.BP_Knight_C|SetCanRoll? _character_2 false)
      (Variables|Default|SetBlockBroken? false))))

(event EventBeginPlay
  (bind _asbp_knight (Utilities|Casting|CastToBP_Knight (Components|GetOwner)))
  (Variables|Default|SetCharacter _asbp_knight))

(fn BlockStartBowType
  (if (Default|HasAmmo1Type? (Variables|/Game/Catalous/Characters/MC/BP_Knight.BP_Knight_C|GetAC_EquipmentSystem (Variables|Default|GetCharacter)))
    (Variables|Default|SetIsBlocking? true)
    (Default|AimBegin (Variables|/Game/Catalous/Characters/MC/BP_Knight.BP_Knight_C|GetAC_BowMechanics (Variables|Default|GetCharacter)))))

(fn BlockStart
  (bind _character (Variables|Default|GetCharacter))
  (switch Utilities|FlowControl|Switch|SwitchonE_WeaponSubtype (Default|GetActiveWeaponType (Variables|Default|GetCharacter))
    (:NewEnumerator0
      (bind _returnvalue (Utilities|GetDataTableRow "/Game/Catalous/Controls/DataTables/DT_WeaponMelee.DT_WeaponMelee" "Fists" :!label _label)
        (:then
          (bind _output_get (Variables|Default|SetCurrentBlockData (Utilities|Struct|BreakS_WeaponMelee _returnvalue)))
          (CallFunction|BlockStartFists _output_get)
          (Variables|Default|SetIsBlocking? true :!label _label_2)
          (Default|SetMovementMode (Variables|Default|GetCharacter) "NewEnumerator1"))))
    (:NewEnumerator1
      (goto _label))
    (:NewEnumerator2
      (bind _asbp_generic_weapon_melee (Utilities|Casting|CastToBP_Generic_Weapon_Melee (Default|GetWeaponActor (Variables|Default|GetCharacter)) :!label _label_3))
      (bind _output_get_2 (Variables|Default|SetCurrentBlockData (Utilities|Struct|BreakS_WeaponMelee (Variables|/Game/Catalous/Weapons/Melee/BP_Generic_Weapon_Melee.BP_Generic_Weapon_Melee_C|GetWeaponData _asbp_generic_weapon_melee))))
      (CallFunction|BlockStartMeleeType _output_get_2)
      (goto _label_2))
    (:NewEnumerator3
      (goto _label_3))
    (:NewEnumerator4
      (if (Default|CanAffordAmount? (Variables|/Game/Catalous/Characters/MC/BP_Knight.BP_Knight_C|GetAC_Stamina _character) (Utilities|Struct|BreakS_WeaponBase (Default|GetActivePrimaryWeapon (Variables|/Game/Catalous/Characters/MC/BP_Knight.BP_Knight_C|GetAC_EquipmentSystem _character))))
        (BlockStart|BlockStartBowType)))))

(fn BlockEnd
  (bind _character (Variables|Default|GetCharacter))
  (bind _subtype (Default|GetActiveWeaponType _character))
  (if (and (not (Default|InAnimationLock? _character)) (Variables|Default|GetIsBlocking?))
    (if (or (Utilities|Enum|Equal(Enum) _subtype "NewEnumerator0") (Utilities|Enum|Equal(Enum) _subtype "NewEnumerator1"))
      (switch Utilities|FlowControl|Switch|SwitchonE_WeaponSubtype (Default|GetActiveWeaponType _character) :!label _label
        (:NewEnumerator0
          (CallFunction|BlockEndFists :!label _label_2)
          (Variables|Default|SetIsBlocking? false :!label _label_3)
          (Default|SetMovementMode (Variables|Default|GetCharacter) "NewEnumerator2"))
        (:NewEnumerator1
          (goto _label_2))
        (:NewEnumerator2
          (CallFunction|BlockEndMeleeType :!label _label_4)
          (goto _label_3))
        (:NewEnumerator3
          (goto _label_4))
        (:NewEnumerator4
          (BlockEnd|BlockEndBowType)
          (Variables|Default|SetIsBlocking? false)))
      (elif (Variables|/Game/Catalous/Components/AC_AttackSystem.AC_AttackSystem_C|GetIsWeaponEquiped? (Variables|/Game/Catalous/Characters/MC/BP_Knight.BP_Knight_C|GetAC_AttackSystem _character))
        (goto _label)))))

(fn BlockEndBowType
  (Default|AimEnd (Variables|/Game/Catalous/Characters/MC/BP_Knight.BP_Knight_C|GetAC_BowMechanics (Variables|Default|GetCharacter)) false))

(fn ParryStart
  (Variables|Default|SetIsParrying? true))

(fn ParryEnd
  (Variables|Default|SetIsParrying? false))