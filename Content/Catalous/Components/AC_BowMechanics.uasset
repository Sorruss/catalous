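; Actor component that runs bow combat for BP_Knight: aiming, drawing, firing and arrow damage.
; Aiming spawns an arrow on the hand socket, and a looping timer accumulates draw time.
; Firing launches it toward the lock-on target or a camera trace point, with normalized draw time setting strength and scaling damage.
; Draw requests that cannot start are queued and resume after the recoil montage if attack is held.
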(event Custom|StopDrawing
  ;[0.15 0.15 0.15 0.5] Drawing Logic
  (CallFunction|ClearDrawingTimer)
  (bind _weapon (Utilities|GetWeaponActor)
    (:execute
      (Default|FireEnd _weapon)
      (Variables|Default|SetIsDrawing? false)
      (Default|CallOnStopDrawing))))

(event Custom|ClearDrawingTimer
  ;[0.15 0.15 0.15 0.5] Drawing Logic
  (if (Utilities|Time|IsValidTimerHandle (stale Custom|StartDrawing _returnvalue))
    (Utilities|Time|ClearandInvalidateTimerbyHandle (stale Custom|StartDrawing _returnvalue))
    (Variables|Default|SetDrawTimeTotal 0.0)))

(event Custom|StartDrawing
  ;[0.15 0.15 0.15 0.5] Drawing Logic
  (Utilities|CanStartDrawing?
    (:Yes
      (Variables|Default|SetQueuedFire? false)
      (Variables|/Game/Catalous/Components/AC_AttackSystem.AC_AttackSystem_C|SetCanDequip? (Variables|/Game/Catalous/Characters/MC/BP_Knight.BP_Knight_C|GetAC_AttackSystem (Variables|Default|GetBP%20Knight)) false)
      (Variables|Default|SetIsDrawing? true)
      (Default|FireBegin (Variables|Default|GetBP%20Weapon))
      (bind _returnvalue (Utilities|Time|SetTimerbyEvent (delegate Custom|IncrementDrawTime) (Variables|Default|GetDrawTimeIncrease) true)))
    (:Nah
      (Variables|Default|SetQueuedFire? true))))

(event Custom|IncrementDrawTime
  ;[0.15 0.15 0.15 0.5] Drawing Logic
  (bind _output_get (Variables|Default|SetDrawTimeTotal (+ (Variables|Default|GetDrawTimeTotal) (Variables|Default|GetDrawTimeIncrease))))
  (Default|CallOnDrawTimeChange _output_get (Utilities|Struct|BreakS_WeaponRanged (Variables|/Game/Catalous/Weapons/Ranged/BP_Generic_Weapon_Ranged.BP_Generic_Weapon_Ranged_C|GetWeaponData (Variables|Default|GetBP%20Weapon)))))

(event Custom|FireBegin
  ;[0.15 0.15 0.15 0.5] Firing Logic
  (Variables|Default|GetAmmoActor
    (:then
      (Variables|Default|SetIsFiring? true)
      (CallFunction|Firing)
      (CallFunction|StopDrawing)
      (CallFunction|FireEnd))
    (:else)))

(event Custom|Firing
  (bind _drawtimetotal (Variables|Default|GetDrawTimeTotal))
  (bind _bp_weapon (Variables|Default|GetBP%20Weapon))
  (bind _weapondata (Variables|/Game/Catalous/Weapons/Ranged/BP_Generic_Weapon_Ranged.BP_Generic_Weapon_Ranged_C|GetWeaponData _bp_weapon))
  (bind _maxdrawtime (Utilities|Struct|BreakS_WeaponRanged _weapondata))
  (bind _returnvalue (Math|Float|NormalizetoRange _drawtimetotal 0.0 _maxdrawtime))
  (bind _returnvalue_2 (Math|Float|Clamp(Float) _returnvalue 0.0 _maxdrawtime))
  ;[0.15 0.15 0.15 0.5] Firing Logic
  (Transformation|DetachFromActor (Variables|Default|GetAmmoActor) "KeepWorld" "KeepWorld" "KeepWorld")
  (CallFunction|UpdateWeapon)
  (Default|Launch (Variables|Default|GetAmmoActor) (CallFunction|GetAmmoLaunchDirection) _returnvalue_2)
  (Variables|Default|SetAmmoActor 0)
  (Variables|Default|SetLastDrawTime _returnvalue_2))

(event Custom|FireEnd
  (bind _bp_knight (Variables|Default|GetBP%20Knight))
  ;[0.15 0.15 0.15 0.5] Firing Logic
  (Animation|Montage|PlayMontage (Variables|/Script/Engine.Character|GetMesh (Variables|Default|GetBP%20Knight)) "/Game/Catalous/Characters/MC/GothicKnight/Animation/Bow/Combat/MDR_standing_aim_recoil_Montage.MDR_standing_aim_recoil_Montage"
    (:then
      (Default|MyMakeNoise (Variables|Default|GetBP%20Knight)))
    (:OnCompleted
      (Variables|Default|SetIsFiring? false :!label _label)
      (if (and (Variables|Default|GetQueuedFire?) (Variables|/Game/Catalous/Characters/MC/BP_Knight.BP_Knight_C|GetHoldingPrimaryAttack? _bp_knight))
        (CallFunction|AimBegin)
        (CallFunction|StartDrawing)
        (Variables|Default|SetQueuedFire? false)
        (else
          (Variables|/Game/Catalous/Components/AC_AttackSystem.AC_AttackSystem_C|SetCanDequip? (Variables|/Game/Catalous/Characters/MC/BP_Knight.BP_Knight_C|GetAC_AttackSystem _bp_knight) true))))
    (:OnInterrupted
      (goto _label))
    (:OnNotifyBegin
      (Variables|Default|SetIsAiming? false))))

(event EventBeginPlay
  (bind _asbp_knight (Utilities|Casting|CastToBP_Knight (Components|GetOwner)))
  (Variables|Default|SetBP%20Knight _asbp_knight)
  (CallFunction|UpdateWeapon))

(fn AimBegin
  (bind _bp_knight (Variables|Default|GetBP%20Knight))
  (if (not (Variables|Default|GetIsFiring?))
    (Default|SetCameraLagSpeed _bp_knight 8.0 false)
    (CallFunction|SetState "NewEnumerator2")
    (Default|AiminBow _bp_knight)
    (CallFunction|SpawnAmmo)
    (Default|CallOnAimBegin)))

(fn AimEnd
  (bind _bp_knight (Variables|Default|GetBP%20Knight))
  (if (not (Variables|/Game/Catalous/Characters/MC/BP_Knight.BP_Knight_C|GetHoldingSecondaryAttack? _bp_knight))
    (Default|SetCameraLagSpeed _bp_knight 0.0 true)
    (Default|AimOutBow _bp_knight)
    (CallFunction|StopDrawing)
    (CallFunction|SetState "NewEnumerator1")
    (Default|CallOnAimEnd)
    (bind _ammoactor (Variables|Default|GetAmmoActor)
      (:then
        (Actor|DestroyActor _ammoactor))
      (:else))))

(fn UpdateWeapon
  (bind _asbp_generic_weapon_ranged (Utilities|Casting|CastToBP_Generic_Weapon_Ranged (Variables|/Game/Catalous/Components/AC_EquipmentSystem.AC_EquipmentSystem_C|GetActiveWeaponActor (Variables|/Game/Catalous/Characters/MC/BP_Knight.BP_Knight_C|GetAC_EquipmentSystem (Variables|Default|GetBP%20Knight)))))
  (Variables|Default|SetBP%20Weapon _asbp_generic_weapon_ranged))

(fn SetState
  (params (NewState :type E_WeaponRangedState%20Enum :default "NewEnumerator0"))
  (Variables|Default|SetIsAiming? (Utilities|Select :Index NewState :NewEnumerator0 false :NewEnumerator1 false :NewEnumerator2 true :NewEnumerator3 true))
  (Variables|Default|SetIsDrawing? (Utilities|Select :Index NewState :NewEnumerator0 false :NewEnumerator1 false :NewEnumerator2 false :NewEnumerator3 true))
  (CallFunction|UpdateWeapon)
  (Class|BPIWeaponRanged|SetState(Message) (Variables|Default|GetBP%20Weapon) NewState))

(fn SpawnAmmo
  (bind _returnvalue (Game|SpawnActorfromClass "/Game/Catalous/Weapons/Ammo/BP_Ammo_DefaultArrow.BP_Ammo_DefaultArrow_C" (Math|Transform|MakeTransform "0, 0, 0" "0, 0, 0" "1.000000,1.000000,1.000000") "AlwaysSpawn" "MultiplyWithRoot" 0 (Variables|Default|GetBP%20Knight)))
  (bind _output_get (Variables|Default|SetAmmoActor _returnvalue))
  (Transformation|AttachComponentToComponent _output_get (Variables|/Script/Engine.Character|GetMesh (Variables|Default|GetBP%20Knight)) "hand_r_arrow" "SnapToTarget" "SnapToTarget" "KeepRelative" true)
  (EventDispatchers|BindEventtoOnHitActor (Variables|Default|GetAmmoActor) (EventDispatchers|CreateEvent :!event DealDamage)))

(fn GetAmmoLaunchDirection
  (bind _bp_knight (Variables|Default|GetBP%20Knight))
  (bind _followcamera (Variables|/Game/Catalous/Characters/MC/BP_Knight.BP_Knight_C|GetFollowCamera _bp_knight))
  (bind _returnvalue (Transformation|GetWorldLocation _followcamera))
  (if (Default|GetIsLockedon (Variables|/Game/Catalous/Characters/MC/BP_Knight.BP_Knight_C|GetAC_TargetingSystem (Variables|Default|GetBP%20Knight)))
    (bind _ammoactor (Variables|Default|GetAmmoActor)
      (:then
        (return (Math|Vector|GetUnitDirection(Vector) (Transformation|GetActorLocation _ammoactor) (Transformation|GetActorLocation (Variables|/Game/Catalous/Components/AC_TargetingSystem.AC_TargetingSystem_C|GetLockedOnActor (Variables|/Game/Catalous/Characters/MC/BP_Knight.BP_Knight_C|GetAC_TargetingSystem (Variables|Default|GetBP%20Knight)))))))
      (:else))
    (else
      (bind (_outhit _returnvalue_2) (Collision|LineTraceByChannel _returnvalue (+ _returnvalue (* (Math|Vector|GetForwardVector _followcamera) 1e+04)) "TraceTypeQuery1" false 0 "None"))
      (bind _ammoactor_2 (Variables|Default|GetAmmoActor)
        (:then
          (return (Math|Vector|GetUnitDirection(Vector) (Transformation|GetActorLocation _ammoactor_2) (Math|Vector|SelectVector (.Location (Collision|BreakHitResult _outhit)) (.TraceEnd (Collision|BreakHitResult _outhit)) _returnvalue_2))))
        (:else)))))

(fn DealDamage
  (params (HitActor :type Actor%20Object%20Reference))
  (bind _bp_weapon (Variables|Default|GetBP%20Weapon))
  (bind _bp_knight (Variables|Default|GetBP%20Knight))
  (bind _lastdrawtime (Variables|Default|GetLastDrawTime))
  (bind _weapondata (Variables|/Game/Catalous/Weapons/Ranged/BP_Generic_Weapon_Ranged.BP_Generic_Weapon_Ranged_C|GetWeaponData _bp_weapon))
  (bind _weaponbase (Utilities|Struct|BreakS_WeaponRanged _weapondata))
  (bind _attackpower (Utilities|Struct|BreakS_WeaponBase _weaponbase))
  (bind _physical (Utilities|Struct|BreakS_AttackPower _attackpower))
  (bind _returnvalue (* _physical _lastdrawtime))
  (Class|BPIDamagable|GetDamaged(Message) HitActor (Utilities|Struct|MakeS_DamageInfo _returnvalue "NewEnumerator2" "NewEnumerator1" false true true true (Variables|Default|GetBP%20Knight)))
  (Class|AISenseDamage|ReportDamageEvent HitActor _bp_knight _returnvalue (Transformation|GetActorLocation _bp_knight) "0, 0, 0" "None"))

(fn SwappedWeapon
  (bind _bp_knight (Variables|Default|GetBP%20Knight))
  (Variables|Default|SetIsAiming? false)
  (Variables|Default|SetIsFiring? false)
  (Variables|Default|SetQueuedFire? false)
  (Variables|Default|SetIsDrawing? false)
  (bind _ammoactor (Variables|Default|GetAmmoActor)
    (:then
      (Actor|DestroyActor _ammoactor))
    (:else
      _))
  (CallFunction|ClearDrawingTimer)
  (Default|AimOutBow _bp_knight)
  (Default|ToggleCameraLag _bp_knight true)
  (Default|CallOnAimEnd))