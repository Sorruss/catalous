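; Bow-combat component for BP_Generic_Enemy that handles aiming, drawing, firing and arrow damage using the enemy's primary ranged weapon.
; Aiming spawns an arrow on the hand socket, and a looping timer accumulates draw time, broadcasting changes.
; Firing detaches and launches the arrow with strength from normalized draw time, then plays a recoil montage.
; DealDamage sends parryable, blockable weapon damage with a hit direction derived from dot products.
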(event Custom|StopDrawing
  ;[0.15 0.15 0.15 0.5] Drawing Logic
  (CallFunction|ClearDrawingTimer)
  (bind _weapon (Utilities|GetWeaponActor)
    (:execute
      (Default|FireEnd _weapon)
      (Variables|Default|SetIsDrawing? false)
      (Default|CallOnStopDrawing))))

(event Custom|ClearDrawingTimer
  ;[0.15 0.15 0.15 0.5] Drawing Logic
  (if (Utilities|Time|IsValidTimerHandle (stale Custom|StartDrawing _returnvalue))
    (Utilities|Time|ClearandInvalidateTimerbyHandle (stale Custom|StartDrawing _returnvalue))
    (Variables|Default|SetDrawTimeTotal 0.0)))

(event Custom|StartDrawing
  ;[0.15 0.15 0.15 0.5] Drawing Logic
  (Utilities|CanStartDrawing?
    (:Yes
      (Variables|Default|SetIsDrawing? true)
      (Default|FireBegin (Variables|Default|GetBP%20Weapon))
      (bind _returnvalue (Utilities|Time|SetTimerbyEvent (delegate Custom|IncrementDrawTime) (Variables|Default|GetDrawTimeIncrease) true)))))

(event Custom|IncrementDrawTime
  ;[0.15 0.15 0.15 0.5] Drawing Logic
  (bind _output_get (Variables|Default|SetDrawTimeTotal (+ (Variables|Default|GetDrawTimeTotal) (Variables|Default|GetDrawTimeIncrease))))
  (Default|CallOnDrawTimeChange _output_get (Utilities|Struct|BreakS_WeaponRanged (Variables|/Game/Catalous/Weapons/Ranged/BP_Generic_Weapon_Ranged.BP_Generic_Weapon_Ranged_C|GetWeaponData (Variables|Default|GetBP%20Weapon)))))

(event Custom|FireBegin
  (params (Direction :type Vector))
  ;[0.15 0.15 0.15 0.5] Firing Logic
  (Variables|Default|GetAmmoActor
    (:then
      (Variables|Default|SetIsFiring? true)
      (CallFunction|Firing Direction)
      (CallFunction|StopDrawing)
      (CallFunction|FireEnd))
    (:else)))

(event Custom|Firing
  (params (Direction :type Vector))
  (bind _bp_weapon (Variables|Default|GetBP%20Weapon))
  (bind _weapondata (Variables|/Game/Catalous/Weapons/Ranged/BP_Generic_Weapon_Ranged.BP_Generic_Weapon_Ranged_C|GetWeaponData _bp_weapon))
  (bind _maxdrawtime (Utilities|Struct|BreakS_WeaponRanged _weapondata))
  ;[0.15 0.15 0.15 0.5] Firing Logic
  (Transformation|DetachFromActor (Variables|Default|GetAmmoActor) "KeepWorld" "KeepWorld" "KeepWorld")
  (CallFunction|UpdateWeapon)
  (Default|Launch (Variables|Default|GetAmmoActor) Direction (Math|Float|Clamp(Float) (Math|Float|NormalizetoRange (Variables|Default|GetDrawTimeTotal) 0.0 _maxdrawtime) 0.0 _maxdrawtime))
  (Variables|Default|SetAmmoActor 0))

(event Custom|FireEnd
  ;[0.15 0.15 0.15 0.5] Firing Logic
  (Animation|Montage|PlayMontage (Variables|/Script/Engine.Character|GetMesh (Variables|Default|GetCharacter)) "/Game/Catalous/Characters/MC/GothicKnight/Animation/Bow/Combat/MDR_standing_aim_recoil_Montage.MDR_standing_aim_recoil_Montage"
    (:OnCompleted
      (Variables|Default|SetIsFiring? false :!label _label))
    (:OnInterrupted
      (goto _label))
    (:OnNotifyBegin
      (Variables|Default|SetIsAiming? false))))

(event EventBeginPlay
  (bind _asbp_generic_enemy (Utilities|Casting|CastToBP_Generic_Enemy (Components|GetOwner)))
  (Variables|Default|SetCharacter _asbp_generic_enemy)
  (CallFunction|UpdateWeapon))

(fn AimBegin
  (if (not (Variables|Default|GetIsFiring?))
    (CallFunction|SetState "NewEnumerator2")
    (CallFunction|SpawnAmmo)
    (Default|CallOnAimBegin)))

(fn AimEnd
  (CallFunction|StopDrawing)
  (CallFunction|SetState "NewEnumerator1")
  (Default|CallOnAimEnd)
  (bind _ammoactor (Variables|Default|GetAmmoActor)
    (:then
      (Actor|DestroyActor _ammoactor))
    (:else)))

(fn UpdateWeapon
  (bind _primaryactor (Class|BPIComponentAI|GetPrimaryasRanged(Message) (Variables|Default|GetCharacter)))
  (Variables|Default|SetBP%20Weapon _primaryactor))

(fn SetState
  (params (NewState :type E_WeaponRangedState%20Enum :default "NewEnumerator0"))
  (Variables|Default|SetIsAiming? (Utilities|Select :Index NewState :NewEnumerator0 false :NewEnumerator1 false :NewEnumerator2 true :NewEnumerator3 true))
  (Variables|Default|SetIsDrawing? (Utilities|Select :Index NewState :NewEnumerator0 false :NewEnumerator1 false :NewEnumerator2 false :NewEnumerator3 true))
  (CallFunction|UpdateWeapon)
  (Class|BPIWeaponRanged|SetState(Message) (Variables|Default|GetBP%20Weapon) NewState))

(fn SpawnAmmo
  (bind _returnvalue (Game|SpawnActorfromClass "/Game/Catalous/Weapons/Ammo/BP_Ammo_DefaultArrow.BP_Ammo_DefaultArrow_C" (Math|Transform|MakeTransform "0, 0, 0" "0, 0, 0" "1.000000,1.000000,1.000000") "AlwaysSpawn" "MultiplyWithRoot" 0 (Variables|Default|GetCharacter)))
  (bind _output_get (Variables|Default|SetAmmoActor _returnvalue))
  (Transformation|AttachComponentToComponent _output_get (Variables|/Script/Engine.Character|GetMesh (Variables|Default|GetCharacter)) "hand_r_arrow" "SnapToTarget" "SnapToTarget" "KeepRelative" true)
  (EventDispatchers|BindEventtoOnHitActor (Variables|Default|GetAmmoActor) (EventDispatchers|CreateEvent :!event DealDamage)))

(fn DealDamage
  (params (HitActor :type Actor%20Object%20Reference))
  (bind _character (Variables|Default|GetCharacter))
  (bind _damagedactorstate (Class|BPIDamagable|GetDamagedActorState(Message) HitActor))
  (Class|BPIDamagable|GetDamaged(Message) HitActor (Utilities|Struct|MakeS_DamageInfo _character (Utilities|Struct|BreakS_AttackPower (Utilities|Struct|BreakS_WeaponBase (Utilities|Struct|BreakS_WeaponRanged (Variables|/Game/Catalous/Weapons/Ranged/BP_Generic_Weapon_Ranged.BP_Generic_Weapon_Ranged_C|GetWeaponData (Variables|Default|GetBP%20Weapon))))) true true true false (CallFunction|GetDirectionOfAnotherActor HitActor _character) _damagedactorstate)))

(fn GetDirectionOfAnotherActor
  (params (TargetActor :type Actor%20Object%20Reference) (AnotherActor :type Actor%20Object%20Reference))
  (bind _returnvalue (Transformation|GetActorForwardVector AnotherActor))
  (bind _returnvalue_2 (Transformation|GetActorForwardVector TargetActor))
  (bind _returnvalue_3 (Transformation|GetActorLocation AnotherActor))
  (bind _returnvalue_4 (Transformation|GetActorLocation TargetActor))
  (bind _returnvalue_5 (Transformation|GetActorRightVector TargetActor))
  (bind _returnvalue_6 (Math|Vector|Normalize _returnvalue))
  (bind _returnvalue_7 (Math|Vector|Normalize _returnvalue_2))
  (bind _returnvalue_8 (- _returnvalue_4 _returnvalue_3))
  (bind _returnvalue_9 (Math|Vector|DotProduct _returnvalue_7 _returnvalue_6))
  (bind _returnvalue_10 (Math|Vector|DotProduct _returnvalue_8 _returnvalue_5))
  (if (>= _returnvalue_9 0.6)
    (LocalVariables|SetReturnValueDirection "NewEnumerator1")
    (elif (<= _returnvalue_9 -0.8)
      (LocalVariables|SetReturnValueDirection "NewEnumerator6")
      (elif (> _returnvalue_10 0.0)
        (LocalVariables|SetReturnValueDirection "NewEnumerator3")
        (elif (< _returnvalue_10 0.0)
          (LocalVariables|SetReturnValueDirection "NewEnumerator2")
          (else
            (LocalVariables|SetReturnValueDirection "NewEnumerator1"))))))
  (return (LocalVariables|GetReturnValueDirection)))