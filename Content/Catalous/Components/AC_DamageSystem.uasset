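; Actor component that manages its owner's health, death, healing and the resolution of incoming hits.
; Health loads from DT_Character by the owner's character name or via SetData, with block cost from DT_MC_Actions.
; GetDamaged uses Damage Scenario to classify hits as damaged, blocked, block-broken, evaded or parried, then fires dispatchers and returns a response.
; Blocked and block-broken hits are reduced by weapon physical stats plus Defense, queried through owner interface messages.
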(event Custom|SetData
  (params (CurrentHealth :type Float%20%28double-precision%29) (MaxHealth :type Float%20%28double-precision%29))
  (Variables|Stat|SetCurrentHealth CurrentHealth)
  (bind _output_get (Variables|Stat|SetMaxHealth MaxHealth))
  (Variables|Stat|SetMaxHealthDefault _output_get)
  (if (< (Variables|Stat|GetCurrentHealth) 0.0)
    (Variables|Status|SetDead? true)
    (else
      (bind _returnvalue (Utilities|GetDataTableRow "/Game/Catalous/Controls/DataTables/DT_MC_Actions.DT_MC_Actions" "Block")
        (:then
          (Variables|Default|SetBlockAction _returnvalue))))))

(event Custom|Data%20injection
  (bind _returnvalue (Components|GetOwner))
  (if (Utilities|DoesObjectImplementInterface _returnvalue "/Game/Catalous/Controls/Interfaces/BPI_Damagable.BPI_Damagable_C")
    (bind _name (Class|BPIDamagable|GetCharacterName(Message) _returnvalue))
    (bind _returnvalue_2 (Utilities|GetDataTableRow "/Game/Catalous/Controls/DataTables/DT_Character.DT_Character" (Utilities|String|StringToName (Utilities|String|EnumtoString _name)))
      (:then
        (Variables|Stat|SetCurrentHealth (.Health (Utilities|Struct|BreakS_Character _returnvalue_2)))
        (bind _output_get (Variables|Stat|SetMaxHealth (.MaxHealth (Utilities|Struct|BreakS_Character _returnvalue_2))))
        (Variables|Stat|SetMaxHealthDefault _output_get)
        (if (< (Variables|Stat|GetCurrentHealth) 0.0)
          (Variables|Status|SetDead? true)
          (else
            (bind _returnvalue_3 (Utilities|GetDataTableRow "/Game/Catalous/Controls/DataTables/DT_MC_Actions.DT_MC_Actions" "Block")
              (:then
                (Variables|Default|SetBlockAction _returnvalue_3)))))))))

(event EventBeginPlay
  (CallFunction|DataInjection))

(fn Heal
  (params (Amount :type Float%20%28double-precision%29))
  (if (and (> Amount 0.0) (not (Variables|Status|GetDead?)))
    (bind _output_get (Variables|Stat|SetCurrentHealth (Math|Float|Clamp(Float) (+ Amount (Variables|Stat|GetCurrentHealth)) (Variables|Stat|GetCurrentHealth) (Variables|Stat|GetMaxHealth))))
    (return true _output_get)
    (else
      (return false (Variables|Stat|GetCurrentHealth)))))

(fn GetDamaged
  (params (DamageInfo :type S%20Damage%20Info%20Structure))
  (bind _damagevalue (Utilities|Struct|BreakS_DamageInfo DamageInfo))
  (Utilities|DamageScenario DamageInfo
    (:Damaged
      (bind _output_get (Variables|Stat|SetCurrentHealth (CallFunction|CountNewHP _damagevalue false)))
      (if (== _output_get 0.0)
        (Variables|Status|SetDead? true)
        (Default|CallOnDeath)
        (return "")
        (else
          (Default|CallOnDamage (Variables|Stat|GetCurrentHealth))
          (return (Utilities|Struct|MakeS_DamagedResponse "NewEnumerator0" (Variables|Stat|GetCurrentHealth))))))
    (:BlockBroke
      (Default|CallOnBlockBreak))
    (:Blocked
      _)
    (:Evaded
      (Default|CallOnEvade)
      (return (Utilities|Struct|MakeS_DamagedResponse "NewEnumerator2" (Variables|Stat|GetCurrentHealth))))
    (:Parried
      (Default|CallOnParry)
      (return (Utilities|Struct|MakeS_DamagedResponse "NewEnumerator3" (Variables|Stat|GetCurrentHealth)))))
  (bind _output_get_2 (Variables|Stat|SetCurrentHealth (CallFunction|CountNewHP _damagevalue true)))
  (if (== _output_get_2 0.0)
    (Variables|Status|SetDead? true)
    (Default|CallOnDeath)
    (return "")
    (else
      (Default|CallOnBlock (Variables|Stat|GetCurrentHealth) (Utilities|GetStaminaReq))
      (return (Utilities|Struct|MakeS_DamagedResponse "NewEnumerator1" (Variables|Stat|GetCurrentHealth))))))

(fn GetHealthRatio
  (return (/ (Variables|Stat|GetCurrentHealth) (Variables|Stat|GetMaxHealth))))

(fn CountNewHP
  (params (Damage :type Float%20%28double-precision%29) (DamageReduction? :type Boolean))
  (bind _defense (Variables|Default|GetDefense))
  (if DamageReduction?
    (bind _damagenegation (Class|BPIDamagable|GetBlockingWeaponStats(Message) (Components|GetOwner)))
    (return (Math|Float|Clamp(Float) (- (Variables|Stat|GetCurrentHealth) (Math|Float|SelectFloat (* Damage (/ (- 1e+02 (Utilities|Struct|BreakS_GuardedDamageNegation _damagenegation)) 1e+02)) (* Damage (/ (- 1e+02 (+ (Utilities|Struct|BreakS_GuardedDamageNegation _damagenegation) _defense)) 1e+02)) (== _defense 0.0))) 0.0 (Variables|Stat|GetMaxHealth)))
    (else
      (return (Math|Float|Clamp(Float) (- (Variables|Stat|GetCurrentHealth) Damage) 0.0 (Variables|Stat|GetMaxHealth))))))

(fn HealPercentage
  (params (AmountPercantage :type Float%20%28double-precision%29))
  (bind _maxhealth (Variables|Stat|GetMaxHealth))
  (if (and (> AmountPercantage 0.0) (not (Variables|Status|GetDead?)))
    (bind _output_get (Variables|Stat|SetCurrentHealth (Math|Float|Clamp(Float) (+ (* (/ AmountPercantage 1e+02) _maxhealth) (Variables|Stat|GetCurrentHealth)) (Variables|Stat|GetCurrentHealth) _maxhealth)))
    (return true _output_get)
    (else
      (return false (Variables|Stat|GetCurrentHealth)))))

(fn IncreaseDefense
  (params (Reset? :type Boolean) (Value :type Float%20%28double-precision%29))
  (Variables|Default|SetDefense (Math|Float|SelectFloat 0.0 (+ Value (Variables|Default|GetDefense)) Reset?)))

(fn SetNewHealth
  (params (Health :type Float%20%28double-precision%29))
  (bind _output_get (Variables|Stat|SetMaxHealth Health))
  (Variables|Stat|SetMaxHealthDefault _output_get))