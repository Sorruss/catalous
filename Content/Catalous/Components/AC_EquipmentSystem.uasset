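; AC_EquipmentSystem is an actor component that creates and toggles the player's equipment screen.
; InitializeWidget creates WBP_Equipment, adds it to the viewport and caches the owning BP_Knight.
; ToggleEquipment plays the widget's in or out animation, waits its length, then switches visibility, cursor, input mode and game pause.
; A CanOpenEquipment flag blocks re-triggering during transitions, and pausing is applied only after the opening animation finishes.
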(event Custom|Toggle%20Equipment
  (bind _returnvalue (Game|GetPlayerController 0))
  (bind _wbp_equipment (Variables|Default|GetWBP%20Equipment))
  ;[0.15 0.15 0.15 0.5] Equipment Widget Toggling Logic
  (if (Variables|Default|GetCan%20Open%20Equipment?)
    (Variables|Default|SetCan%20Open%20Equipment? false)
    (if (Widget|IsVisible _wbp_equipment)
      (Game|SetGamePaused false)
      (bind _time_to_animate (Default|AnimationOut _wbp_equipment))
      (Variables|/Script/Engine.PlayerController|SetbShowMouseCursor (Game|GetPlayerController 0) false)
      (Utilities|FlowControl|Delay _time_to_animate)
      (Widget|SetVisibility _wbp_equipment "Hidden")
      (Input|SetInputModeGameOnly _returnvalue false)
      (Variables|Default|SetCan%20Open%20Equipment? true)
      (else
        (Widget|SetVisibility _wbp_equipment "Visible")
        (bind _time_to_animate_2 (Default|Animationin _wbp_equipment))
        (Variables|/Script/Engine.PlayerController|SetbShowMouseCursor (Game|GetPlayerController 0) true)
        (Utilities|FlowControl|Delay _time_to_animate_2)
        (Input|SetInputModeGameandUI _returnvalue (Variables|Default|GetWBP%20Equipment) "DoNotLock" false false)
        (Variables|Default|SetCan%20Open%20Equipment? true)
        (Game|SetGamePaused true)))))

(fn InitializeWidget
  (bind _returnvalue (UserInterface|CreateWidget "/Game/Catalous/UI/WBP_Equipment.WBP_Equipment_C" (Game|GetPlayerController 0)))
  (bind _output_get (Variables|Default|SetWBP%20Equipment _returnvalue))
  (UserInterface|Viewport|AddtoViewport _output_get 0)
  (bind _asbp_knight (Utilities|Casting|CastToBP_Knight (Components|GetOwner)))
  (Variables|Default|SetBP%20Knight _asbp_knight))