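; Inventory component for BP_Knight that stores melee weapons, ranged weapons and consumables and toggles an animated inventory widget that pauses the game.
; AddItem box-traces through the knight's bounds, reads the hit pickup's category and data via interface messages, then destroys it.
; Weapons receive random IDs for later lookup, while consumables stack by identifier.
; SetItemInSlot passes weapons to AC_EquipmentSystem slots and adjusts the carried load by item weight.
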(event Custom|Toggle%20Inventory
  (bind _returnvalue (Game|GetPlayerController 0))
  (bind _wbp_inventory (Variables|Default|GetWBP%20Inventory))
  ;[0.15 0.15 0.15 0.5] Inventory Widget Toggling Logic
  (if (Variables|Default|GetCanOpenInventory?)
    (Variables|Default|SetCanOpenInventory? false)
    (if (Widget|IsVisible _wbp_inventory)
      (Game|SetGamePaused false)
      (bind _timetoanimate (Default|AnimationOut _wbp_inventory))
      (Variables|/Script/Engine.PlayerController|SetbShowMouseCursor (Game|GetPlayerController 0) false)
      (Utilities|FlowControl|Delay _timetoanimate)
      (Widget|SetVisibility _wbp_inventory "Hidden")
      (Input|SetInputModeGameOnly _returnvalue false)
      (Variables|Default|SetCanOpenInventory? true)
      (else
        (Default|UpdateConsumables _wbp_inventory (Variables|Default|GetConsumables))
        (Widget|SetVisibility _wbp_inventory "Visible")
        (bind _timetoanimate_2 (Default|Animationin _wbp_inventory))
        (Variables|/Script/Engine.PlayerController|SetbShowMouseCursor (Game|GetPlayerController 0) true)
        (Utilities|FlowControl|Delay _timetoanimate_2)
        (Input|SetInputModeGameandUI _returnvalue (Variables|Default|GetWBP%20Inventory) "DoNotLock" false false)
        (Variables|Default|SetCanOpenInventory? true)
        (Game|SetGamePaused true)))))

(fn AddItem
  (bind _bp_knight (Variables|Default|GetBP%20Knight))
  (bind (_origin _boxextent) (Collision|GetActorBounds _bp_knight true false))
  (bind (_outhit _returnvalue) (Class|KismetSystemLibrary|BoxTraceSingleforObjects (Math|Vector|MakeVector (.x _origin) (.y _origin) (+ (.z _origin) (.z _boxextent))) (Math|Vector|MakeVector (.x _origin) (.y _origin) (- (.z _origin) (.z _boxextent))) "35.000000,35.000000,35.000000" "0, 0, 0" (Utilities|Array|MakeArray "ObjectTypeQuery8") false 0 "None" true))
  (if _returnvalue
    (bind _category (Class|BPIPickable|GetCategory(Message) (.HitActor (Collision|BreakHitResult _outhit))))
    (switch Utilities|FlowControl|Switch|SwitchonE_Item_Category _category
      (:NewEnumerator1
        (bind _data (Class|BPIPickable|GetWeaponMeleeData(Message) (.HitActor (Collision|BreakHitResult _outhit))))
        (Adding|AddWeaponMelee _data))
      (:NewEnumerator4
        (bind _data_2 (Class|BPIPickable|GetConsumableData(Message) (.HitActor (Collision|BreakHitResult _outhit))))
        (Adding|AddConsumable _data_2))
      (:NewEnumerator6
        (bind _data_3 (Class|BPIPickable|GetWeaponRangedData(Message) (.HitActor (Collision|BreakHitResult _outhit))))
        (Adding|AddRangedWeapon _data_3)))
    (Actor|DestroyActor (.HitActor (Collision|BreakHitResult _outhit)))
    (return true)
    (else
      (return false))))

(fn AddWeaponMelee
  (params (Data :type S%20Weapon%20Melee%20Structure))
  (bind _weaponbase (Utilities|Struct|BreakS_WeaponMelee Data))
  (bind _structout (Utilities|Struct|SetmembersinS_ItemBase (.ItemBase (Utilities|Struct|BreakS_WeaponBase _weaponbase)) (Math|Random|RandomIntegerinRange 100000 2147483640)))
  (bind _structout_2 (Utilities|Struct|SetmembersinS_WeaponBase _weaponbase _structout))
  (bind _structout_3 (Utilities|Struct|SetmembersinS_WeaponMelee Data _structout_2))
  (Utilities|Array|Add (Variables|Default|GetWeaponsMelee) _structout_3))

(fn AddConsumable
  (params (Data :type S%20Consumables%20Structure%20%28by%20ref%29))
  (bind (_identifier _quantity) (Utilities|Struct|BreakS_Consumables Data))
  (bind _consumables (Variables|Default|GetConsumables))
  (for (_array_element _array_index) _consumables
    (if (Utilities|Enum|Equal(Enum) (.Identifier (Utilities|Struct|BreakS_Consumables _array_element)) _identifier)
      (bind _structout (Utilities|Struct|SetmembersinS_Consumables _array_element (+ (.Quantity (Utilities|Struct|BreakS_Consumables _array_element)) _quantity)))
      (Utilities|Array|SetArrayElem (Variables|Default|GetConsumables) _array_index _structout)
      (return)))
  (Utilities|Array|Add _consumables Data)
  (return))

(fn InitializeWidget
  (bind _returnvalue (UserInterface|CreateWidget "/Game/Catalous/UI/WBP_Inventory.WBP_Inventory_C" (Game|GetPlayerController 0)))
  (bind _output_get (Variables|Default|SetWBP%20Inventory _returnvalue))
  (UserInterface|Viewport|AddtoViewport _output_get 0)
  (bind _asbp_knight (Utilities|Casting|CastToBP_Knight (Components|GetOwner)))
  (Variables|Default|SetBP%20Knight _asbp_knight)
  (Default|UpdateConsumables (Variables|Default|GetWBP%20Inventory) (Variables|Default|GetConsumables)))

(fn SetIteminSlot
  (params (SlotCategory :type E_Item_Category%20Enum :default "NewEnumerator0") (SlotIndex :type Integer) (ItemId :type Integer))
  (bind _bp_knight (Variables|Default|GetBP%20Knight))
  (bind _ac_equipmentsystem (Variables|/Game/Catalous/Characters/MC/BP_Knight.BP_Knight_C|GetAC_EquipmentSystem _bp_knight))
  (bind _data (CallFunction|GetWeaponbyId ItemId))
  (switch Utilities|FlowControl|Switch|SwitchonE_Item_Category SlotCategory
    (:NewEnumerator1
      (bind _id (Default|GetWeaponIdSlot _ac_equipmentsystem SlotIndex))
      (bind (_data_2 _success_) (CallFunction|GetWeaponbyId _id))
      (if _success_
        (CallFunction|ReduceLoad (Utilities|Struct|BreakS_ItemBase (Utilities|Struct|BreakS_WeaponBase _data_2))))
      (bind _addtoloadvalue (Default|SetWeaponSlot _ac_equipmentsystem SlotIndex ItemId (.Icon (Utilities|Struct|BreakS_ItemBase (Utilities|Struct|BreakS_WeaponBase _data)))))
      (if _addtoloadvalue
        (Variables|Default|SetLoadValue (+ (Variables|Default|GetLoadValue) (.Weight (Utilities|Struct|BreakS_ItemBase (Utilities|Struct|BreakS_WeaponBase _data)))))))))

(fn GetWeaponbyId
  (params (Id :type Integer))
  (for _array_element (Variables|Default|GetWeaponsMelee)
    (if (== (Utilities|Struct|BreakS_ItemBase (Utilities|Struct|BreakS_WeaponBase (Utilities|Struct|BreakS_WeaponMelee _array_element))) Id)
      (return (Utilities|Struct|BreakS_WeaponMelee _array_element) true)))
  (for _array_element_2 (Variables|Default|GetWeaponsRanged)
    (if (== (Utilities|Struct|BreakS_ItemBase (Utilities|Struct|BreakS_WeaponBase (Utilities|Struct|BreakS_WeaponRanged _array_element_2))) Id)
      (return (Utilities|Struct|BreakS_WeaponRanged _array_element_2) true)))
  (return "" false))

(fn ReduceLoad
  (params (Amount :type Float%20%28double-precision%29))
  (Variables|Default|SetLoadValue (Math|Float|Clamp(Float) (- (Variables|Default|GetLoadValue) Amount) 0.0 (- (Variables|Default|GetLoadValue) Amount))))

(fn AddRangedWeapon
  (params (Data :type S%20Weapon%20Ranged%20Structure))
  (bind _weaponbase (Utilities|Struct|BreakS_WeaponRanged Data))
  (bind _structout (Utilities|Struct|SetmembersinS_ItemBase (Utilities|Struct|BreakS_WeaponBase _weaponbase) (Math|Random|RandomIntegerinRange 100000 2147483640)))
  (bind _structout_2 (Utilities|Struct|SetmembersinS_WeaponBase _weaponbase _structout))
  (bind _structout_3 (Utilities|Struct|SetmembersinS_WeaponRanged Data _structout_2))
  (Utilities|Array|Add (Variables|Default|GetWeaponsRanged) _structout_3))

(fn GetWeaponsCategory
  (for _array_element (Variables|Default|GetWeaponsMelee)
    (Utilities|Array|Add (LocalVariables|GetResult) (Utilities|Struct|BreakS_WeaponMelee _array_element)))
  (for _array_element_2 (Variables|Default|GetWeaponsRanged)
    (Utilities|Array|Add (LocalVariables|GetResult) (Utilities|Struct|BreakS_WeaponRanged _array_element_2)))
  (return (LocalVariables|GetResult)))

(fn GetWeaponMelee
  (params (ID :type Integer))
  (for _array_element (Variables|Default|GetWeaponsMelee)
    (if (== (Utilities|Struct|BreakS_ItemBase (Utilities|Struct|BreakS_WeaponBase (Utilities|Struct|BreakS_WeaponMelee _array_element))) ID)
      (return _array_element true)))
  (return "" false))