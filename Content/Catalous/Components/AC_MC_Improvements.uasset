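; Player progression component for BP_Knight that runs bonfire rests, warping, and souls-based leveling.
; Bonfire interaction locks input, shows the menu, plays sit/stand montages, resets stats and signals an enemy reset through the GameInstance.
; Warps teleport within the level or save and open another level.
; Souls convert to levels and upgrade points on a breakpoint cost curve; Strength, Endurance and Intelligence scale DataTable base stats and max load.
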(event Custom|InteractionBonfire
  (params (Location :type Vector))
  (bind _returnvalue (Game|GetPlayerController 0))
  (bind _character (Variables|Default|GetCharacter))
  (bind _character_2 (Variables|Default|GetCharacter))
  (Components|Movement|StopMovementImmediately (Variables|/Script/Engine.Character|GetCharacterMovement _character_2))
  (Variables|Default|SetAtBonfire? true)
  (Default|AnimationLock _character_2 true)
  (Input|SetInputModeUIOnly _returnvalue (Variables|Default|GetWBP%20Bonfire) "DoNotLock" false)
  (Variables|/Script/Engine.PlayerController|SetbShowMouseCursor _returnvalue true)
  (Transformation|SetActorRotation _character_2 (Math|Rotator|FindLookatRotation (Transformation|GetActorLocation _character_2) Location))
  (Default|Show (Variables|Default|GetWBP%20Bonfire))
  (Default|ShowInteractTip _character_2 "NewEnumerator2" false)
  (Default|ToggleHUD _character_2 false)
  (Utilities|FlowControl|Delay 0.5)
  (Default|EquipInstant (Variables|/Game/Catalous/Characters/MC/BP_Knight.BP_Knight_C|GetAC_AttackSystem (Variables|Default|GetCharacter)) true)
  (Animation|Montage|PlayMontage (Variables|/Script/Engine.Character|GetMesh (Variables|Default|GetCharacter)) "/Game/Catalous/Characters/MC/GothicKnight/Animation/Other/Sitting_Idle_Montage.Sitting_Idle_Montage"
    (:then
      (Class|BPISaveGame|ResetEnemies(Message) (Game|GetGameInstance))
      (Default|ResetStats _character)
      (Audio|PlaySound2D "/Game/Catalous/SFX/UI/Menu/finger.finger" 1.0 1.0 0.0 0 0)
      (Default|HealthChanged _character)
      (Default|StaminaChanged _character))))

(event Custom|BonfireExit
  (bind _returnvalue (Game|GetPlayerController 0))
  (bind _character (Variables|Default|GetCharacter))
  (bind _character_2 (Variables|Default|GetCharacter))
  (bind _animinstance (Variables|/Game/Catalous/Characters/MC/BP_Knight.BP_Knight_C|GetAnimInstance _character_2))
  (Variables|/Script/Engine.PlayerController|SetbShowMouseCursor _returnvalue false)
  (Default|ToggleHUD _character true)
  (bind _notifyname (Animation|Montage|PlayMontage (Variables|/Script/Engine.Character|GetMesh _character) "/Game/Catalous/Characters/MC/GothicKnight/Animation/Other/Stand_Up_Montage.Stand_Up_Montage" 1.25)
    (:then
      (Input|SetInputModeGameOnly _returnvalue true))
    (:OnNotifyBegin
      (switch name _notifyname
        (:AnimationLockOff
          (Default|AnimationLock _character_2 false)
          (Variables|Default|SetAtBonfire? false)
          (Animation|Montage|MontageStop _animinstance 0.0 (Animation|Montage|GetCurrentActiveMontage _animinstance)))))))

(event Custom|WarpTo
  (params (BonfireData :type S%20Bonfire%20Structure%20%28by%20ref%29))
  (bind _spawntransform (Utilities|Struct|BreakS_Bonfire BonfireData))
  (Default|Show (Variables|Default|GetWBP%20Bonfire))
  (Utilities|FlowControl|Delay 0.5)
  (Transformation|SetActorLocationAndRotation (Variables|Default|GetCharacter) (.location _spawntransform) (.rotation _spawntransform))
  (Class|BPISaveGame|SetPlayerSave(Message) (Game|GetGameInstance) (Default|GetPlayerSave (Variables|Default|GetCharacter)) true)
  (Audio|PlaySound2D "/Game/Catalous/SFX/UI/Menu/warping.warping" 0.15 1.0 0.0 0 0))

(event Custom|WarpToAnotherLevel
  (params (LevelName :type E_LevelNames%20Enum :default "NewEnumerator0") (DestWarpName :type E_WarpNames%20Enum :default "NewEnumerator0"))
  (bind _returnvalue (Game|GetGameInstance))
  (bind _character (Variables|Default|GetCharacter))
  (Default|ToggleHUD _character false)
  (Default|ShowInteractTip _character "NewEnumerator3" false)
  (Class|BPIGameInstance|SetDestWarpName(Message) _returnvalue DestWarpName)
  (Class|BPIGameInstance|SetLevelName(Message) _returnvalue LevelName)
  (Class|BPISaveGame|SaveGameData(Message) _returnvalue true)
  (Default|Show (Variables|Default|GetWBP%20Bonfire))
  (Utilities|FlowControl|Delay 0.5)
  (Game|OpenLevel(byName) (Utilities|String|StringToName (Utilities|String|EnumtoString LevelName)))
  (Audio|PlaySound2D "/Game/Catalous/SFX/UI/Menu/warping.warping" 0.15 1.0 0.0 0 0))

(event EventBeginPlay
  (bind _asbp_knight (Utilities|Casting|CastToBP_Knight (Game|Player|GetPlayerPawn 0)))
  (Variables|Default|SetCharacter _asbp_knight)
  (bind _returnvalue (UserInterface|CreateWidget "/Game/Catalous/UI/WBP_Bonfire.WBP_Bonfire_C" (Game|GetPlayerController 0)))
  (bind _output_get (Variables|Default|SetWBP%20Bonfire _returnvalue))
  (UserInterface|Viewport|AddtoViewport _output_get 0)
  (bind _returnvalue_2 (UserInterface|CreateWidget "/Game/Catalous/UI/WBP_WarpMenu.WBP_WarpMenu_C" (Game|GetPlayerController 0)))
  (bind _output_get_2 (Variables|Default|SetWBP%20Warp _returnvalue_2))
  (UserInterface|Viewport|AddtoViewport _output_get_2 0)
  (bind _returnvalue_3 (Utilities|GetDataTableRow "/Game/Catalous/Controls/DataTables/DT_Character.DT_Character" "MC")
    (:then
      (Variables|Default|SetDefaultCharacter _returnvalue_3)
      (Variables|Default|SetMaxLoad (Variables|Default|GetDefaultMaxLoad)))))

(fn GainSouls
  (params (Souls :type Integer))
  (bind _structout (Utilities|Struct|SetmembersinS_LevelUpData (Variables|Default|GetLevelUpData) (+ Souls (Utilities|Struct|BreakS_LevelUpData (Variables|Default|GetLevelUpData)))))
  (Variables|Default|SetLevelUpData _structout)
  (Default|SetSoulsCounter (Variables|/Game/Catalous/Characters/MC/BP_Knight.BP_Knight_C|GetWBP%20HUD (Variables|Default|GetCharacter)) (Utilities|Struct|BreakS_LevelUpData (Variables|Default|GetLevelUpData)))
  (CallFunction|UpdateEquipmentUI))

(fn ShowWarpMenu?
  (params (Show? :type Boolean))
  (Widget|SetVisibility (Variables|Default|GetWBP%20Warp) (select Show? "Visible" "Visible")))

(fn UpdateEquipmentUI
  (Default|UpdateMCStats (Variables|/Game/Catalous/Components/AC_EquipmentSystem.AC_EquipmentSystem_C|GetWBP%20Equipment (Variables|/Game/Catalous/Characters/MC/BP_Knight.BP_Knight_C|GetAC_EquipmentSystem (Variables|Default|GetCharacter)))))

(fn GainPoints
  (bind _souls (CallFunction|CalculateSoulsforNextLevel))
  (bind _levelupdata (Variables|Default|GetLevelUpData))
  (bind (_level _upgradepoints _souls_2) (Utilities|Struct|BreakS_LevelUpData _levelupdata))
  (while (>= _souls_2 _souls)
    (Utilities|Struct|SetmembersinS_LevelUpData (Variables|Default|GetLevelUpData) (+ _level 1) (+ _upgradepoints 1) (- _souls_2 _souls)))
  (Default|SavePlayerSave (Variables|Default|GetCharacter) true))

(fn CalculateSoulsforNextLevel
  (bind _levelupdata (Variables|Default|GetLevelUpData))
  (bind _startingcostofpoint (Variables|Default|GetStartingCostOfPoint))
  (bind _level (Utilities|Struct|BreakS_LevelUpData _levelupdata))
  (if (< _level (Variables|Default|GetLevelBreakpoint))
    (return (+ _startingcostofpoint (Math|Float|Truncate (* _startingcostofpoint _level 0.832))))
    (else
      (return (Math|Float|Truncate (- (+ (+ (* (* (* _level _level) _level) 0.02) (* (* _level _level) 2.06)) (* _level 85.6)) 895.0))))))

(fn Improve
  (params (NewData :type S%20Level%20Up%20Data%20Structure))
  (bind _character (Variables|Default|GetCharacter))
  (bind _defaultcharacter (Variables|Default|GetDefaultCharacter))
  (bind _defaultmaxload (Variables|Default|GetDefaultMaxLoad))
  (bind (_maxhealth _maxstamina _maxmana) (Utilities|Struct|BreakS_Character _defaultcharacter))
  (bind _output_get (Variables|Default|SetLevelUpData NewData))
  (bind _structout (Utilities|Struct|SetmembersinS_Character (Variables|/Game/Catalous/Characters/MC/BP_Knight.BP_Knight_C|GetCharacterStruct (Variables|Default|GetCharacter)) (+ _maxhealth (* _maxhealth (.Strength (Utilities|Struct|BreakS_LevelUpData _output_get)) 0.1)) (+ _maxstamina (* _maxstamina (.Endurance (Utilities|Struct|BreakS_LevelUpData _output_get)) 0.05)) (+ _maxmana (* _maxmana (.Intelligence (Utilities|Struct|BreakS_LevelUpData _output_get)) 0.1))))
  (Default|SavePlayerSave _character true)
  (Variables|Default|SetMaxLoad (+ _defaultmaxload (* _defaultmaxload (.Strength (Utilities|Struct|BreakS_LevelUpData _output_get)) (.Endurance (Utilities|Struct|BreakS_LevelUpData _output_get)) 0.01)))
  (Default|SetNewStamina (Variables|/Game/Catalous/Characters/MC/BP_Knight.BP_Knight_C|GetAC_Stamina _character) (.MaxStamina (Utilities|Struct|BreakS_Character _structout)))
  (Default|SetNewHealth (Variables|/Game/Catalous/Characters/MC/BP_Knight.BP_Knight_C|GetAC_DamageSystem _character) (.MaxHealth (Utilities|Struct|BreakS_Character _structout)))
  (Default|UpdateMCStats (Variables|/Game/Catalous/Components/AC_EquipmentSystem.AC_EquipmentSystem_C|GetWBP%20Equipment (Variables|/Game/Catalous/Characters/MC/BP_Knight.BP_Knight_C|GetAC_EquipmentSystem _character)))
  (Default|ResetStats _character))

(fn UseSaved
  (params (NewData :type S%20Level%20Up%20Data%20Structure))
  (bind _defaultcharacter (Variables|Default|GetDefaultCharacter))
  (bind _defaultmaxload (Variables|Default|GetDefaultMaxLoad))
  (bind (_maxhealth _maxstamina _maxmana) (Utilities|Struct|BreakS_Character _defaultcharacter))
  (bind _output_get (Variables|Default|SetLevelUpData NewData))
  (Utilities|Struct|SetmembersinS_Character (Variables|/Game/Catalous/Characters/MC/BP_Knight.BP_Knight_C|GetCharacterStruct (Variables|Default|GetCharacter)) (+ _maxhealth (* _maxhealth (.Strength (Utilities|Struct|BreakS_LevelUpData _output_get)) 0.1)) (+ _maxstamina (* _maxstamina (.Endurance (Utilities|Struct|BreakS_LevelUpData _output_get)) 0.05)) (+ _maxmana (* _maxmana (.Intelligence (Utilities|Struct|BreakS_LevelUpData _output_get)) 0.1)))
  (Variables|Default|SetMaxLoad (+ _defaultmaxload (* _defaultmaxload (.Strength (Utilities|Struct|BreakS_LevelUpData _output_get)) (.Endurance (Utilities|Struct|BreakS_LevelUpData _output_get)) 0.01))))