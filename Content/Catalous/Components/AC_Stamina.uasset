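; Actor component that manages a character's stamina pool, spending it on actions and attacks and regenerating it over time.
; On BeginPlay, owners implementing BPI_Damagable load stats and movement speeds from DT_Character by character name, and action costs from DT_MC_Actions into a map.
; Spending checks affordability, then restarts a delayed looping regen timer that stops at max.
; Functions raise or reset max stamina, and changes fire a StaminaChanged dispatcher.
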(event Custom|Stamina%20Regeneration
  ;[0.15 0.15 0.15 0.5] Stamina Regen Logic
  (bind _returnvalue (Utilities|Time|SetTimerbyEvent (delegate Custom|Add%20Stamina) (Variables|Stamina|GetStaminaRegenPer) true)))

(event Custom|Data%20injection
  (bind _returnvalue (Components|GetOwner))
  ;[0.15 0.15 0.15 0.5] Data Injection
  (if (Utilities|DoesObjectImplementInterface _returnvalue "/Game/Catalous/Controls/Interfaces/BPI_Damagable.BPI_Damagable_C")
    (bind _name (Class|BPIDamagable|GetCharacterName(Message) _returnvalue))
    (bind _returnvalue_2 (Utilities|GetDataTableRow "/Game/Catalous/Controls/DataTables/DT_Character.DT_Character" (Utilities|String|StringToName (Utilities|String|EnumtoString _name)))
      (:then
        (Variables|Movement|SetWalkSpeed (.WalkSpeed (Utilities|Struct|BreakS_Character _returnvalue_2)))
        (Variables|Movement|SetJogSpeed (.JogSpeed (Utilities|Struct|BreakS_Character _returnvalue_2)))
        (Variables|Movement|SetRunSpeed (.RunSpeed (Utilities|Struct|BreakS_Character _returnvalue_2)))
        (Variables|Stamina|SetCurrentStamina (.Stamina (Utilities|Struct|BreakS_Character _returnvalue_2)))
        (bind _output_get (Variables|Stamina|SetMaxStamina (.MaxStamina (Utilities|Struct|BreakS_Character _returnvalue_2))))
        (Variables|Stamina|SetMaxStaminaDefault _output_get)
        (bind _output_get_2 (Variables|Stamina|SetStaminaRegen (.StaminaRegen (Utilities|Struct|BreakS_Character _returnvalue_2))))
        (Variables|Stamina|SetStaminaRegenDefault _output_get_2)
        (bind _outrownames (DataTable|GetDataTableRowNames "/Game/Catalous/Controls/DataTables/DT_MC_Actions.DT_MC_Actions"))
        (for _array_element _outrownames
          (bind _returnvalue_3 (Utilities|GetDataTableRow "/Game/Catalous/Controls/DataTables/DT_MC_Actions.DT_MC_Actions" _array_element)
            (:then
              (Utilities|Map|Add (Variables|Default|GetActionsCost) (.Action (Utilities|Struct|BreakS_MC_Actions _returnvalue_3)) (Utilities|Struct|MakeS_MC_Actions (.Action (Utilities|Struct|BreakS_MC_Actions _returnvalue_3)) (.StaminaCost (Utilities|Struct|BreakS_MC_Actions _returnvalue_3)) (.HealthCost (Utilities|Struct|BreakS_MC_Actions _returnvalue_3)) (.ManaCost (Utilities|Struct|BreakS_MC_Actions _returnvalue_3)))))))))))

(event Custom|Add%20Stamina
  (bind _maxstamina (Variables|Stamina|GetMaxStamina))
  ;[0.15 0.15 0.15 0.5] Stamina Regen Logic
  (if (not (== (Math|Float|Clamp(Float) (+ (Variables|Stamina|GetCurrentStamina) (Variables|Stamina|GetStaminaRegen)) 0.0 _maxstamina) _maxstamina))
    (Variables|Stamina|SetCurrentStamina (Math|Float|Clamp(Float) (+ (Variables|Stamina|GetCurrentStamina) (Variables|Stamina|GetStaminaRegen)) 0.0 _maxstamina))
    (else
      (Variables|Stamina|SetCurrentStamina _maxstamina)
      (CallFunction|StopStaminaRegeneration)))
  (Default|CallStaminaChanged))

(event Custom|Stop%20Stamina%20Regeneration
  ;[0.15 0.15 0.15 0.5] Stamina Regen Logic
  (if (Utilities|Time|IsValidTimerHandle (stale Custom|Stamina%20Regeneration _returnvalue))
    (Utilities|Time|ClearandInvalidateTimerbyHandle (stale Custom|Stamina%20Regeneration _returnvalue))
    (if (< (Variables|Stamina|GetCurrentStamina) (Variables|Stamina|GetMaxStamina))
      (Utilities|Time|SetTimerbyEvent (delegate Custom|Stamina%20Regeneration) (Variables|Stamina|GetStamineRegenTimeout) :!label _label))
    (else
      (goto _label))))

(event EventBeginPlay
  (CallFunction|DataInjection))

(fn CanAfford?
  (params (Action :type E_MC_Actions%20Enum :default "NewEnumerator0"))
  (bind _actionscost (Variables|Default|GetActionsCost))
  (bind (_value _returnvalue) (Utilities|Map|Find _actionscost Action))
  (if _returnvalue
    (return (>= (- (Variables|Stamina|GetCurrentStamina) (Utilities|Struct|BreakS_MC_Actions _value)) 0.0))))

(fn UseStamina
  (params (Action :type E_MC_Actions%20Enum :default "NewEnumerator0"))
  (if (CallFunction|CanAfford? Action)
    (Variables|Stamina|SetCurrentStamina (- (Variables|Stamina|GetCurrentStamina) (Utilities|Struct|BreakS_MC_Actions (.Value (Utilities|Map|Find (Variables|Default|GetActionsCost) Action)))))
    (CallFunction|StopStaminaRegeneration)
    (Default|CallStaminaChanged)
    (return true)
    (else
      (return false))))

(fn GetStaminaRatio
  (return (/ (Variables|Stamina|GetCurrentStamina) (Variables|Stamina|GetMaxStamina))))

(fn UseStaminaAttack
  (params (Amount :type Float%20%28double-precision%29))
  (if (CallFunction|CanAffordAmount? Amount)
    (Variables|Stamina|SetCurrentStamina (- (Variables|Stamina|GetCurrentStamina) Amount))
    (CallFunction|StopStaminaRegeneration)
    (Default|CallStaminaChanged)
    (return true)
    (else
      (return false))))

(fn CanAffordAmount?
  (params (Amount :type Float%20%28double-precision%29))
  (return (>= (- (Variables|Stamina|GetCurrentStamina) Amount) 0.0)))

(fn IncreaseStaminaMax
  (params (ToDefault? :type Boolean) (IncreaseValue :type Float%20%28double-precision%29))
  (Variables|Stamina|SetMaxStamina (Math|Float|SelectFloat (Variables|Stamina|GetMaxStaminaDefault) (+ IncreaseValue (Variables|Stamina|GetMaxStamina)) ToDefault?))
  (Default|CallStaminaChanged)
  (CallFunction|StaminaRegeneration))

(fn IncreaseStaminaMaxPercentage
  (params (ToDefault? :type Boolean) (IncreaseValuePercentage :type Float%20%28double-precision%29))
  (Variables|Stamina|SetMaxStamina (Math|Float|SelectFloat (Variables|Stamina|GetMaxStaminaDefault) (* (/ (+ IncreaseValuePercentage 1e+02) 1e+02) (Variables|Stamina|GetMaxStamina)) ToDefault?))
  (Default|CallStaminaChanged)
  (CallFunction|StaminaRegeneration))