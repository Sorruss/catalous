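; Lock-on targeting component for BP_Knight that acquires, switches and releases enemy targets.
; A sphere trace ahead of the camera gathers living BPI_Targetable actors in clear sight; Fire picks the nearest, while FireDirectional switches left or right using camera-right dot products.
; While locked, Tick interpolates controller yaw toward the target and movement follows controller rotation, with a special bow camera offset.
; Turn-in-place montage logic exists but is disconnected.
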(event Custom|PlayTurnInPlaceMontage
  (params (NewParam :type E_CDirection%20Enum :default "NewEnumerator0"))
  ;[0.15 0.15 0.15 0.5] For future maybe?
  (if (not (Utilities|Enum|Equal(Enum) NewParam (Variables|Default|GetPrevTurnInSide)))
    (Animation|PlayAnimMontage (Variables|Default|GetBP%20Knight) (Utilities|Select :Index NewParam :NewEnumerator0 0 :NewEnumerator1 0 :NewEnumerator2 "/Game/Catalous/Characters/MC/GothicKnight/Animation/Unarmed/Turn/Left_Turn_Montage.Left_Turn_Montage" :NewEnumerator3 0 :NewEnumerator4 "/Game/Catalous/Characters/MC/GothicKnight/Animation/Unarmed/Turn/Right_Turn_Montage.Right_Turn_Montage") 1.0 "None")
    (Variables|Default|SetPrevTurnInSide NewParam :!label _label)
    (elif (Utilities|Enum|Equal(Enum) NewParam "NewEnumerator1")
      (Animation|StopAnimMontage (Variables|Default|GetBP%20Knight) (Utilities|Select :Index (Variables|Default|GetPrevTurnInSide) :NewEnumerator0 0 :NewEnumerator1 0 :NewEnumerator2 "/Game/Catalous/Characters/MC/GothicKnight/Animation/Unarmed/Turn/Left_Turn_Montage.Left_Turn_Montage" :NewEnumerator3 0 :NewEnumerator4 "/Game/Catalous/Characters/MC/GothicKnight/Animation/Unarmed/Turn/Right_Turn_Montage.Right_Turn_Montage"))
      (goto _label))))

(event Custom|LockedOnValueChange
  ;[0.15 0.15 0.15 0.5] Camera Control Rotation
  (if (Variables|Default|GetLockedOn?)
    (Utilities|FlowControl|Gate true) ; enters at Open
    (else
      (Utilities|FlowControl|Gate true) ; enters at Close
    )))

(event EventBeginPlay
  ;[0.15 0.15 0.15 0.5] Data Injection
  (bind _asbp_knight (Utilities|Casting|CastToBP_Knight (Components|GetOwner)))
  (bind _output_get (Variables|Default|SetBP%20Knight _asbp_knight))
  (Variables|Default|SetAC%20Camera (Actor|GetComponentbyClass _output_get "/Script/Engine.CameraComponent")))

(event EventTick
  (params (DeltaSeconds :type Float%20%28single-precision%29))
  ;[0.15 0.15 0.15 0.5] Camera Control Rotation
  (Utilities|FlowControl|Gate true
    (:Exit
      (bind _ratio (Class|BPICommonUI|GetHealthRatio(Message) (Variables|Default|GetLockedOnActor)))
      (if (!= _ratio 0.0)
        (CallFunction|FaceActor)
        (else
          (CallFunction|LockOff))))))

(fn TrytoFindTargets
  (bind _sphereradius (Variables|Default|GetSphereRadius))
  (bind _foundactors (LocalVariables|GetFoundActors))
  (bind _bp_knight (Variables|Default|GetBP%20Knight))
  (bind _ac_camera (Variables|Default|GetAC%20Camera))
  (bind _returnvalue (Transformation|GetActorLocation _bp_knight))
  (bind _returnvalue_2 (Math|Vector|GetForwardVector _ac_camera))
  (bind _returnvalue_3 (* (Math|Vector|MakeVector (.x _returnvalue_2) (.y _returnvalue_2) 0.0) _sphereradius))
  (bind _returnvalue_4 (+ _returnvalue _returnvalue_3))
  (bind (_outhits _returnvalue_5) (Collision|MultiSphereTraceForObjects _returnvalue_4 _returnvalue_4 _sphereradius (Utilities|Array|MakeArray "ObjectTypeQuery7") false 0 "None"))
  (if _returnvalue_5
    (for _array_element _outhits
      (bind _ratio (Class|BPICommonUI|GetHealthRatio(Message) (.HitActor (Collision|BreakHitResult _array_element))))
      (if (Math|Boolean|ANDBoolean (!= _ratio 0.0) (Utilities|DoesObjectImplementInterface (.HitActor (Collision|BreakHitResult _array_element)) "/Game/Catalous/Controls/Interfaces/BPI_Targetable.BPI_Targetable_C") (not (CallFunction|IsObjectBetweenActors? (Variables|Default|GetBP%20Knight) (.HitActor (Collision|BreakHitResult _array_element)))))
        (Utilities|Array|Add (LocalVariables|GetFoundActors) (.HitActor (Collision|BreakHitResult _array_element)))))
    (return (> (Utilities|Array|Length _foundactors) 0) _foundactors)
    (else
      (return false 0))))

(fn Fire
  (params (Direction :type E_CDirection%20Enum :default "NewEnumerator0"))
  (bind (_targetsfound_ _actors) (CallFunction|TrytoFindTargets))
  (bind (_targetsfound__2 _actors_2) (CallFunction|TrytoFindTargets))
  (bind _actor (CallFunction|GetClosestActor _actors_2))
  (bind _actor_2 (CallFunction|GetClosestActorDirectional _actors Direction))
  (if (or (not (Variables|Default|GetLockedOn?)) (Variables|Default|GetIsDirectional?))
    (if (Variables|Default|GetIsDirectional?)
      ;[0.15 0.15 0.15 0.5] C - Switch Lock On Target
      (if (and _targetsfound_ (Utilities|IsValid _actor_2))
        (Class|BPITargetable|ShowLockonWidget(Message) (Variables|Default|GetLockedOnActor) false)
        (Class|BPITargetable|ShowHealthBarWidget(Message) (Variables|Default|GetLockedOnActor) false true)
        (Variables|Default|SetLockedOnActor _actor_2)
        (CallFunction|Lockon)
        (return true)
        (else
          (return false)))
      (else
        ;[0.15 0.15 0.15 0.5] A - Lock On Target
        (if (and _targetsfound__2 (Utilities|IsValid _actor))
          (Variables|Default|SetLockedOnActor _actor)
          (CallFunction|Lockon)
          (return true)
          (else
            (return false)))))
    (else
      (CallFunction|LockOff))))

(fn GetClosestActor
  (params (Actors :type Array%20of%20Actor%20Object%20References))
  (LocalVariables|SetClosestDistance (* (Variables|Default|GetSphereRadius) 2.5))
  (for _array_element Actors
    (if (< (Transformation|GetDistanceTo (Variables|Default|GetBP%20Knight) _array_element) (LocalVariables|GetClosestDistance))
      (LocalVariables|SetClosestDistance (Transformation|GetDistanceTo (Variables|Default|GetBP%20Knight) _array_element))
      (LocalVariables|SetClosestActor _array_element)))
  (return (LocalVariables|GetClosestActor)))

(fn Lockon
  (bind _lockedonactor (Variables|Default|GetLockedOnActor))
  (bind _bp_knight (Variables|Default|GetBP%20Knight))
  (Variables|Default|SetLockedOn? true)
  (CallFunction|LockedonValueChange)
  (CallFunction|Activate8Way true)
  (Class|BPITargetable|ShowLockonWidget(Message) _lockedonactor true)
  (Class|BPITargetable|ShowHealthBarWidget(Message) _lockedonactor true true)
  (if (Utilities|Enum|Equal(Enum) (Default|GetActiveWeaponType (Variables|Default|GetBP%20Knight)) "NewEnumerator4")
    (Default|SetBoomOffset _bp_knight (Variables|/Game/Catalous/Components/AC_BowMechanics.AC_BowMechanics_C|GetCameraOffsetLockOn (Variables|/Game/Catalous/Characters/MC/BP_Knight.BP_Knight_C|GetAC_BowMechanics _bp_knight)))
    (Default|CallOnLockon)))

(fn IsObjectBetweenActors?
  (params (Actor1 :type Actor%20Object%20Reference) (Actor2 :type Actor%20Object%20Reference))
  (bind _returnvalue (Collision|LineTraceByChannel (Transformation|GetActorLocation Actor1) (Transformation|GetActorLocation Actor2) "TraceTypeQuery1" false (Utilities|Array|MakeArray Actor2) "None"))
  (if _returnvalue
    (return true)
    (else
      (return false))))

(fn Activate8Way
  (params (Activate? :type Boolean))
  (bind _bp_knight (Variables|Default|GetBP%20Knight))
  (bind _returnvalue (Actor|GetComponentbyClass _bp_knight "/Script/Engine.CharacterMovementComponent"))
  (Utilities|IsValid _returnvalue
    (:Is%20Valid
      (Variables|/Script/Engine.CharacterMovementComponent|SetbUseControllerDesiredRotation _returnvalue Activate?)
      (Variables|/Script/Engine.CharacterMovementComponent|SetbOrientRotationToMovement _returnvalue (not Activate?)))))

(fn FaceActor
  (bind _bp_knight (Variables|Default|GetBP%20Knight))
  (bind _returnvalue (Pawn|GetController _bp_knight))
  (bind _returnvalue_2 (Pawn|GetControlRotation _returnvalue :!class /Script/Engine.Controller))
  (Pawn|SetControlRotation _returnvalue (Math|Interpolation|RInterpTo (Math|Rotator|MakeRotator (.roll _returnvalue_2) (.pitch _returnvalue_2) (.yaw _returnvalue_2)) (Math|Rotator|MakeRotator (.roll _returnvalue_2) (.pitch _returnvalue_2) (.yaw (Math|Rotator|FindLookatRotation (Transformation|GetActorLocation _bp_knight) (Transformation|GetActorLocation (Variables|Default|GetLockedOnActor))))) (Utilities|Time|GetWorldDeltaSeconds) (Variables|Default|GetCamera%20Align%20Speed))))

(fn GetIsLockedon
  (return (Variables|Default|GetLockedOn?)))

(fn FireDirectional
  (params (Direction :type E_CDirection%20Enum :default "NewEnumerator0"))
  (Variables|Default|SetIsDirectional? true)
  (CallFunction|Fire Direction)
  (Variables|Default|SetIsDirectional? false))

(fn GetClosestActorDirectional
  (params (Actors :type Array%20of%20Actor%20Object%20References) (Direction :type E_CDirection%20Enum :default "NewEnumerator0"))
  (LocalVariables|SetClosestDP (.RawResult (CallFunction|GetSideBasedonActor (Variables|Default|GetLockedOnActor))))
  (for _array_element Actors
    (if (not (== _array_element (Variables|Default|GetLockedOnActor)))
      (switch Utilities|FlowControl|Switch|SwitchonE_CDirection (.Side (CallFunction|GetSideBasedonActor _array_element))
        (:NewEnumerator2
          (if (and (< (LocalVariables|GetClosestDP) (.RawResult (CallFunction|GetSideBasedonActor _array_element))) (Utilities|Enum|Equal(Enum) (.Side (CallFunction|GetSideBasedonActor _array_element)) Direction))
            (return _array_element)))
        (:NewEnumerator4
          (if (and (> (LocalVariables|GetClosestDP) (.RawResult (CallFunction|GetSideBasedonActor _array_element))) (Utilities|Enum|Equal(Enum) (.Side (CallFunction|GetSideBasedonActor _array_element)) Direction))
            (return _array_element))))))
  (return 0))

(fn GetSideBasedonActor
  (params (Actor :type Actor%20Object%20Reference))
  (bind _returnvalue (Transformation|GetActorLocation Actor))
  (bind _bp_knight (Variables|Default|GetBP%20Knight))
  (bind _ac_camera (Variables|Default|GetAC%20Camera))
  (bind _returnvalue_2 (Transformation|GetActorLocation _bp_knight))
  (bind _returnvalue_3 (Math|Vector|GetRightVector _ac_camera))
  (bind _returnvalue_4 (- _returnvalue_2 _returnvalue))
  (bind _returnvalue_5 (Math|Vector|Normalize _returnvalue_4))
  (bind _returnvalue_6 (Math|Vector|DotProduct _returnvalue_3 _returnvalue_5))
  (if (< _returnvalue_6 0.0)
    (return "NewEnumerator4" _returnvalue_6)
    (else
      (return "NewEnumerator2" _returnvalue_6))))

(fn LockOff
  (bind _bp_knight (Variables|Default|GetBP%20Knight))
  (bind _lockedonactor (Variables|Default|GetLockedOnActor))
  (bind _defaultcameraoffset (Variables|/Game/Catalous/Characters/MC/BP_Knight.BP_Knight_C|GetDefaultCameraOffset _bp_knight))
  (CallFunction|Activate8Way false)
  (Variables|Default|SetLockedOn? false)
  (CallFunction|LockedonValueChange)
  (Class|BPITargetable|ShowLockonWidget(Message) _lockedonactor false)
  (Class|BPITargetable|ShowHealthBarWidget(Message) _lockedonactor false true)
  (if (Class|KismetMathLibrary|NotEqualExactlyVectorVector (Variables|/Script/Engine.SpringArmComponent|GetSocketOffset (Variables|/Game/Catalous/Characters/MC/BP_Knight.BP_Knight_C|GetCameraBoom _bp_knight)) _defaultcameraoffset)
    (Default|SetBoomOffset (Variables|Default|GetBP%20Knight) _defaultcameraoffset)
    (Default|CallOnLockOff)))

(fn CalculateRotateDirection
  (bind _output_get (LocalVariables|SetDotProduct (Math|Vector|DotProduct (Math|Vector|GetRightVector (Variables|Default|GetAC%20Camera)) (Transformation|GetActorForwardVector (Variables|Default|GetBP%20Knight)))))
  (if (or (> _output_get (Math|Float|Absolute(Float) (LocalVariables|GetSens))) (< (LocalVariables|GetDotProduct) (LocalVariables|GetSens)))
    (if (> (LocalVariables|GetDotProduct) (Math|Float|Absolute(Float) (LocalVariables|GetSens)))
      (return "NewEnumerator2")
      (else
        (return "NewEnumerator4")))
    (else
      (return "NewEnumerator1"))))

(fn GetPitchTowardsEnemy
  (bind _lockedonactor (Variables|Default|GetLockedOnActor))
  (return (.pitch (Math|Rotator|Delta(Rotator) (Math|Rotator|FindLookatRotation (Transformation|GetActorLocation (Variables|Default|GetBP%20Knight)) (Transformation|GetActorLocation _lockedonactor)) (Transformation|GetActorRotation _lockedonactor)))))