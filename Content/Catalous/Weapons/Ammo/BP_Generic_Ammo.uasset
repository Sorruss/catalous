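; Base ammo projectile that is launched, reports what it hits through OnHitActor and makes impact sound, noise and VFX.
; Launch first line-traces along the ammo to land on any blocking actor immediately, otherwise it adds a projectile movement component with Strength-scaled speed and gravity.
; Land stops movement, pushes physics bodies, and destroys the ammo on skeletal-mesh actors or otherwise leaves it for a set lifespan, attached unless it hit other ammo.
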(event OnComponentBeginOverlap(CollisionSphere)
  (params (OverlappedComponent :type Primitive%20Component%20Object%20Reference) (OtherActor :type Actor%20Object%20Reference) (OtherComp :type Primitive%20Component%20Object%20Reference) (OtherBodyIndex :type Integer) (bFromSweep :type Boolean) (SweepResult :type Hit%20Result%20Structure%20%28by%20ref%29))
  (bind (_bblockinghit _binitialoverlap _time _distance _location _impactpoint _normal _impactnormal _physmat _hitactor _hitcomponent) (Collision|BreakHitResult SweepResult))
  (CallFunction|Land _hitactor _hitcomponent))

(event EventBeginPlay
  (Collision|SetCollisionEnabled (Variables|Default|GetCollisionSphere) "NoCollision"))

(fn ConstructionScript)

(fn Launch
  (params (Direction :type Vector) (Strength :type Float%20%28double-precision%29))
  (bind (_hit_ _actor _component) (CallFunction|CheckifActorinBetween))
  (if _hit_
    (Audio|PlaySoundatLocation (Variables|Default|GetFireSC) (Transformation|GetActorLocation) "0, 0, 0" 1.0 1.0 0.0 0 0 0 0)
    (CallFunction|Land _actor _component)
    (else
      (Collision|SetCollisionEnabled (Variables|Default|GetCollisionSphere) "QueryAndPhysics")
      (bind _returnvalue (AddComponent|AddProjectileMovementComponent))
      (bind _output_get (Variables|/Script/Engine.MovementComponent|SetVelocity _returnvalue (* Direction (Math|Float|Lerp (Variables|Default|GetMinSpeed) (Variables|Default|GetMaxSpeed) Strength))))
      (Variables|Default|SetAmmoVelocity _output_get)
      (Variables|/Script/Engine.ProjectileMovementComponent|SetProjectileGravityScale _returnvalue (Math|Float|Lerp (Variables|Default|GetMaxGravity) (Variables|Default|GetMinGravity) Strength))
      (Variables|Default|SetPMComponent _returnvalue)
      (Audio|PlaySoundatLocation (Variables|Default|GetFireSC) (Transformation|GetActorLocation) "0, 0, 0" 1.0 1.0 0.0 0 0 0 0)
      (bind _returnvalue_2 (Niagara|SpawnSystemAttached (Variables|Default|GetAmmoTrail) (Variables|Default|GetAmmoTrailSpawn) "None" "0, 0, 0" "0, 0, 0" "KeepRelativeOffset" false))
      (Variables|Default|SetAmmoTrailRef _returnvalue_2))))

(fn CheckifActorinBetween
  (bind (_outhit _returnvalue) (Collision|LineTraceByChannel (Transformation|GetWorldLocation (Variables|Default|GetAmmoTrailSpawn)) (Transformation|GetWorldLocation (Variables|Default|GetAmmoEnd)) "TraceTypeQuery1" false (Utilities|Array|MakeArray (Variables|Actor|GetInstigator)) "None"))
  (if _returnvalue
    (return true (.HitActor (Collision|BreakHitResult _outhit)) (.HitComponent (Collision|BreakHitResult _outhit)))
    (else
      (return false 0 0))))

(fn Land
  (params (Actor :type Actor%20Object%20Reference) (Component :type Primitive%20Component%20Object%20Reference))
  (bind _returnvalue (Transformation|GetActorLocation))
  (if (!= Actor (Variables|Actor|GetInstigator))
    (bind _pmcomponent (Variables|Default|GetPMComponent)
      (:then
        (Components|DestroyComponent _pmcomponent))
      (:else
        _))
    (Utilities|IsValid (Actor|GetComponentbyClass Actor "/Script/Engine.SkeletalMeshComponent")
      (:Is%20Valid
        (Variables|Default|SetShoudBeDestroyed? true))
      (:Is%20Not%20Valid
        (if (Utilities|ClassIsChildOf (Utilities|GetClass Actor) "BP_Generic_Ammo_C")
          _
          (else
            (Transformation|AttachComponentToComponent Component "None" "KeepWorld" "KeepWorld" "KeepWorld" true)))))
    (if (Physics|IsSimulatingPhysics Component "None")
      (Physics|AddImpulse Component (Variables|Default|GetAmmoVelocity) "None" true))
    (bind _ammotrailref (Variables|Default|GetAmmoTrailRef)
      (:then
        (Components|DestroyComponent _ammotrailref))
      (:else
        _))
    (Audio|PlaySoundatLocation (Variables|Default|GetImpactSC) _returnvalue "0, 0, 0" 1.0 1.0 0.0 0 0 0 0)
    (Class|Actor|MakeNoise 1.0 0 _returnvalue 0.0 "None")
    (Effects|SpawnEmitteratLocation (Variables|Default|GetImpactVFX) (Transformation|GetWorldLocation (Variables|Default|GetVFXSpawn)) "0, 0, 0" "0.250000,0.250000,0.250000")
    (Default|CallOnHitActor Actor)
    (if (Variables|Default|GetShoudBeDestroyed?)
      (Actor|DestroyActor)
      (Variables|Default|SetShoudBeDestroyed? false)
      (else
        (Actor|SetLifeSpan (Variables|Default|GetAmmoLifespan))
        (bind _collisionsphere (Variables|Default|GetCollisionSphere)
          (:then
            (Components|DestroyComponent _collisionsphere))
          (:else))))))