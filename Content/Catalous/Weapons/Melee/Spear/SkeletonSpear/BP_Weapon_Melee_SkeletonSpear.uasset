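; BP_Weapon_Melee_SkeletonSpear is a melee spear weapon Blueprint that supplies mesh and socket data to its parent class.
; It returns WeaponMesh and the world locations of its Tip and Bottom sockets as trace endpoints.
; It also names a separate socket pair for the weapon trail and caches all of the mesh's socket names after the parent SetSockets runs.
; BeginPlay and construction only call the parent.
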(event EventBeginPlay
  (|CallParentFunction))

(fn ConstructionScript
  (|CallParentFunction))

(fn GetTraceSocketsLocation
  (bind _weaponmesh (Variables|Default|GetWeaponMesh))
  (return (Transformation|GetSocketLocation _weaponmesh "Tip") (Transformation|GetSocketLocation _weaponmesh "Bottom")))

(fn GetMesh
  (return (Variables|Default|GetWeaponMesh)))

(fn SetSockets
  (|CallParentFunction)
  (Variables|Default|SetSockets (Transformation|GetAllSocketNames (Variables|Default|GetWeaponMesh))))

(fn GetTrailSockets
  (return "Socket" "Socket_10"))