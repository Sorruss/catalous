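; Generic ranged weapon Blueprint that holds weapon data, a state and firing audio.
; On BeginPlay it looks up its DT_WeaponRanged row using the WeaponName enum as the row name and stores it as WeaponData.
; FireBegin and FireEnd switch the state enum and start or stop a fire sound spawned at the weapon's location.
; SetState allows setting the state directly; no projectile or hit logic is implemented here.
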(event Custom|FireBegin
  (Variables|Default|SetState "NewEnumerator3")
  (bind _returnvalue (Audio|SpawnSoundatLocation (Variables|Default|GetFireSC) (Transformation|GetActorLocation) "0, 0, 0" 1.0 1.0 0.0 0 0)))

(event Custom|FireEnd
  (Variables|Default|SetState "NewEnumerator1")
  (Utilities|IsValid (stale Custom|FireBegin _returnvalue)
    (:Is%20Valid
      (Audio|Components|Audio|Stop (stale Custom|FireBegin _returnvalue)))))

(event EventBeginPlay
  (|CallParentFunction)
  (bind _returnvalue (Utilities|GetDataTableRow "/Game/Catalous/Controls/DataTables/DT_WeaponRanged.DT_WeaponRanged" (Utilities|String|StringToName (Utilities|String|EnumtoString (Variables|Default|GetWeaponName))))
    (:then
      (Variables|Default|SetWeaponData _returnvalue))))

(event EventSetState
  (params (NewState :type E_WeaponRangedState%20Enum :default "NewEnumerator0"))
  (Variables|Default|SetState NewState))

(fn ConstructionScript
  (|CallParentFunction))