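; BP_Skeleton_Body is a modular skeleton body for the Skeleton Guard, assembled from separate bone-part meshes such as skull, jaw, limbs and collarbones.
; The construction script sets the main Mesh as leader pose component for every part, so they all follow one pose.
; SimulatePhysics switches on physics for the main Mesh and all parts together.
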(fn ConstructionScript
  (Components|SkinnedMesh|SetLeaderPoseComponent (Variables|Default|GetSKM_Skeleton_Lord_Body_Skull) (Variables|Character|GetMesh) false false))

(fn SimulatePhysics
  (Physics|SetSimulatePhysics (Variables|Character|GetMesh) true))